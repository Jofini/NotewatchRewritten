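; Notebook actor that the player raises and lowers, animated through its skeletal mesh.
; NBCall and NBFall play notebook and page-turn sounds at random pitch, then run the same animation forward from the start or backward from the end.
; Every tick it looks up the first-person character and copies its base aim rotation, so the notebook turns with the camera.
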(event Custom|NBCall
  (bind _nb_skele (Variables|Default|GetNB_Skele))
  ;[1 0.7782 0.3906 0.5] NBCall
  (Audio|PlaySound2D "/Game/NotewatchContent/Audio/Sounds/Notebook.Notebook" 1.0 (Math|Random|RandomFloatinRange 0.75 1.25) 0.0 0 0)
  (Audio|PlaySound2D "/Game/NotewatchContent/Audio/Sounds/PageTurn.PageTurn" 1.0 (Math|Random|RandomFloatinRange 0.75 1.25) 0.0 0 0)
  (Audio|Components|Audio|Play _nb_skele false)
  (Components|Animation|SetPosition _nb_skele 0.0 true)
  (Components|Timeline|SetPlayRate _nb_skele 0.75))

(event Custom|NBFall
  (bind _nb_skele (Variables|Default|GetNB_Skele))
  ;[0.3333 0.4633 1 0.5] NBFall
  (Audio|PlaySound2D "/Game/NotewatchContent/Audio/Sounds/Notebook.Notebook" 1.0 (Math|Random|RandomFloatinRange 0.75 1.25) 0.0 0 0)
  (Audio|PlaySound2D "/Game/NotewatchContent/Audio/Sounds/PageTurn.PageTurn" 1.0 (Math|Random|RandomFloatinRange 0.75 1.25) 0.0 0 0)
  (Audio|Components|Audio|Play _nb_skele false)
  (Components|Animation|SetPosition _nb_skele 1.0 true)
  (Components|Timeline|SetPlayRate _nb_skele -0.75))

(event EventBeginPlay)

(event EventTick
  (params (DeltaSeconds :type Float%20%28single-precision%29))
  ;[0.8389 0.5581 1 0.5] Rotates With Camera
  (bind _returnvalue (Actor|GetActorOfClass "/Game/FirstPerson/Blueprints/BP_FirstPersonCharacter.BP_FirstPersonCharacter_C"))
  (Transformation|SetActorRotation (Pawn|GetBaseAimRotation _returnvalue)))

(fn ConstructionScript)