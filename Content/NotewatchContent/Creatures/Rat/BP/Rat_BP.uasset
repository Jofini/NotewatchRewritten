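; Rat creature Blueprint that makes a rat periodically scurry out from one of three preset spots, unless it is fleeing.
; SHOW waits a random delay, teleports the actor to a random start transform, then plays Niagara and a random attenuated rustle sound.
; It eases the animated skeletal mesh to the matching show transform with MoveComponentTo, then calls itself to loop.
; Nothing in this graph calls SHOW initially or sets the fleeing flag.
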(event Custom|SHOW
  (bind _skeletalmesh (Variables|Default|GetSkeletalMesh))
  (bind _skeletalmesh_2 (Variables|Default|GetSkeletalMesh))
  ;[1 0.2527 0.8639] SHOW
  (if (not (Variables|Default|GetRatFLEEING))
    (Components|Activation|Deactivate (Variables|Default|GetNiagara))
    (Utilities|FlowControl|Delay (Math|Random|RandomFloatinRange 1.0 15.0))
    (Components|Animation|PlayAnimation _skeletalmesh "/Game/NotewatchContent/Creatures/Rat/Other/Rat_Anim.Rat_Anim" true)
    (Components|Timeline|SetPlayRate _skeletalmesh 4.0)
    (switch int (Math|Random|RandomIntegerinRange 0 2)
      (:0
        (Variables|Default|SetStartLOC (Variables|Default|GetLOC1))
        (Variables|Default|SetLOCShow (Variables|Default|GetLOC1Show))
        (Variables|Default|SetStartROT (Variables|Default|GetROT1))
        (Variables|Default|SetStartROTShow (Variables|Default|GetROT1Show)))
      (:1
        (Variables|Default|SetStartLOC (Variables|Default|GetLOC2))
        (Variables|Default|SetLOCShow (Variables|Default|GetLOC2Show))
        (Variables|Default|SetStartROT (Variables|Default|GetROT2))
        (Variables|Default|SetStartROTShow (Variables|Default|GetROT2Show)))
      (:2
        (Variables|Default|SetStartLOC (Variables|Default|GetLOC3))
        (Variables|Default|SetLOCShow (Variables|Default|GetLOC3Show))
        (Variables|Default|SetStartROT (Variables|Default|GetROT3))
        (Variables|Default|SetStartROTShow (Variables|Default|GetROT3Show))))
    (Transformation|SetActorLocationAndRotation (Variables|Default|GetStartLOC) (Variables|Default|GetStartROT) false true)
    (Components|Activation|Activate (Variables|Default|GetNiagara) false)
    (Utilities|FlowControl|Delay 0.25)
    ;;[0 0 0 0.5] Sound
    (Audio|PlaySoundatLocation (.OutItem (Utilities|Array|Random (Utilities|Array|MakeArray "/Game/NotewatchContent/Audio/Sounds/Rustle1.Rustle1" "/Game/NotewatchContent/Audio/Sounds/Rustle2.Rustle2" "/Game/NotewatchContent/Audio/Sounds/Rustle3.Rustle3"))) "0, 0, 0" "0, 0, 0" (Math|Random|RandomFloatinRange 0.5 0.5) (Math|Random|RandomFloatinRange 2.0 2.0) 0.0 "/Game/NotewatchContent/Audio/Sounds/RinglingerAmbientAtten.RinglingerAmbientAtten" 0 0 0)
    (Components|MoveComponentTo _skeletalmesh_2 (Variables|Default|GetLOCShow) (Variables|Default|GetStartROTShow) true true (Math|Random|RandomFloatinRange 2.5 3.5) true)
    (Components|Animation|PlayAnimation _skeletalmesh_2 "/Game/NotewatchContent/Creatures/Rat/Other/Rat_Anim.Rat_Anim" true)
    (Components|Timeline|SetPlayRate _skeletalmesh_2 2.0)
    (Components|Activation|Deactivate (Variables|Default|GetNiagara))
    (CallFunction|SHOW)))

(fn ConstructionScript)