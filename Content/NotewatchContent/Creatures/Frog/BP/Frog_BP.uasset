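; Ambient frog creature that periodically leaps away, hides and reappears at one of three preset spots.
; FLEE arcs it to FleeLOC with jump animation and rustle sounds, teleports it far below, waits, then picks a new spot.
; Chained MoveComponentTo moves animate each hop; after landing it idles for a random time before fleeing again.
; SHOW triggers a delayed appearance unless fleeing, and Tick uses a random Delay for positional ribbits.
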(event Custom|FLEE
  (bind _skeletalmesh (Variables|Default|GetSkeletalMesh))
  (bind _skeletalmesh_2 (Variables|Default|GetSkeletalMesh))
  (bind _defsceneroot (Variables|Default|GetDefSceneRoot))
  (bind _defsceneroot_2 (Variables|Default|GetDefSceneRoot))
  (bind _skeletalmesh_3 (Variables|Default|GetSkeletalMesh))
  (bind _returnvalue (Transformation|GetWorldLocation _defsceneroot_2))
  (bind _returnvalue_2 (Transformation|GetWorldRotation _defsceneroot))
  ;[0 0.2291 1] FLEE
  (Utilities|FlowControl|Sequence
    (:then_0
      (goto _label Stop))
    (:then_1
      (if (not (Variables|Default|GetFrogFLEEING))
        (Variables|Default|SetFrogFLEEING true)
        (Components|MoveComponentTo _defsceneroot (Variables|Default|GetStartLOC) (Math|Rotator|MakeRotator (.roll _returnvalue_2) (.pitch _returnvalue_2) -1.5e+02) true true 1.0 true)
        ;;[0 0 0 0.5] Sound
        (Audio|PlaySoundatLocation "/Game/NotewatchContent/Audio/Sounds/Frog.Frog" _returnvalue "0, 0, 0" (Math|Random|RandomFloatinRange 0.5 1.0) (Math|Random|RandomFloatinRange 0.5 2.0) 0.0 "/Game/NotewatchContent/Audio/Sounds/RinglingerAmbientAtten.RinglingerAmbientAtten" 0 0 0)
        (Components|Animation|PlayAnimation _skeletalmesh "/Game/NotewatchContent/Creatures/Frog/Other/Jump.Jump" true)
        (Components|Timeline|SetPlayRate _skeletalmesh 0.5)
        (Components|MoveComponentTo (Variables|Default|GetDefSceneRoot) (+ (Variables|Default|GetFleeLOC) "-50.000000,-50.000000,750.000000") (Math|Rotator|MakeRotator -45.0 0.0 -1.5e+02) true false 0.35 true)
        (Components|MoveComponentTo (Variables|Default|GetDefSceneRoot) (Variables|Default|GetFleeLOC) (Math|Rotator|MakeRotator -9e+01 0.0 -1.5e+02) false true 0.35 true)
        ;;[0 0 0 0.5] Sound
        (Audio|PlaySoundatLocation (.OutItem (Utilities|Array|Random (Utilities|Array|MakeArray "/Game/NotewatchContent/Audio/Sounds/Rustle1.Rustle1" "/Game/NotewatchContent/Audio/Sounds/Rustle2.Rustle2" "/Game/NotewatchContent/Audio/Sounds/Rustle3.Rustle3"))) _returnvalue "0, 0, 0" (Math|Random|RandomFloatinRange 0.25 0.5) (Math|Random|RandomFloatinRange 1.75 2.0) 0.0 "/Game/NotewatchContent/Audio/Sounds/RinglingerAmbientAtten.RinglingerAmbientAtten" 0 0 0)
        (Variables|Default|SetStartLOC "0.000000,0.000000,-50000.000000")
        (Transformation|SetWorldLocation (Variables|Default|GetDefSceneRoot) (Variables|Default|GetStartLOC) false true)
        (Transformation|SetActorLocation (Variables|Default|GetStartLOC) false true)
        (Utilities|FlowControl|Delay (Math|Random|RandomFloatinRange 1.0 3e+01))
        (Variables|Default|SetFrogFLEEING false)
        ;[1 0.2527 0.8639] SHOW
        (Components|Animation|PlayAnimation _skeletalmesh_2 "/Game/NotewatchContent/Creatures/Frog/Other/Jump.Jump" true)
        (Components|Timeline|SetPlayRate _skeletalmesh_2 2.0)
        (switch int (Math|Random|RandomIntegerinRange 0 2)
          (:0
            (Variables|Default|SetStartLOC (Variables|Default|GetLOC1))
            (Variables|Default|SetStartROT (Variables|Default|GetROT1)))
          (:1
            (Variables|Default|SetStartLOC (Variables|Default|GetLOC2))
            (Variables|Default|SetStartROT (Variables|Default|GetROT2)))
          (:2
            (Variables|Default|SetStartLOC (Variables|Default|GetLOC3))
            (Variables|Default|SetStartROT (Variables|Default|GetROT3))))
        (Transformation|SetActorLocationAndRotation (- (Variables|Default|GetStartLOC) "300.000000,10.000000,300.000000") (Math|Rotator|MakeRotator 9e+01 (.pitch (Variables|Default|GetStartROT)) (.yaw (Variables|Default|GetStartROT))) false true)
        ;;[0 0 0 0.5] Sound
        (Audio|PlaySoundatLocation (.OutItem (Utilities|Array|Random (Utilities|Array|MakeArray "/Game/NotewatchContent/Audio/Sounds/Rustle1.Rustle1" "/Game/NotewatchContent/Audio/Sounds/Rustle2.Rustle2" "/Game/NotewatchContent/Audio/Sounds/Rustle3.Rustle3"))) _returnvalue "0, 0, 0" (Math|Random|RandomFloatinRange 0.25 0.5) (Math|Random|RandomFloatinRange 1.75 2.0) 0.0 "/Game/NotewatchContent/Audio/Sounds/RinglingerAmbientAtten.RinglingerAmbientAtten" 0 0 0)
        (Components|MoveComponentTo (Variables|Default|GetDefSceneRoot) (- (Variables|Default|GetStartLOC) "0.000000,0.000000,-100.000000") (Variables|Default|GetStartROT) true false 0.5 true)
        (Components|MoveComponentTo (Variables|Default|GetDefSceneRoot) (Variables|Default|GetStartLOC) (Variables|Default|GetStartROT) false true 0.5 true :!label _label)
        (Components|Animation|PlayAnimation _skeletalmesh_3 "/Game/NotewatchContent/Creatures/Frog/Other/Idle.Idle" true)
        (Components|Timeline|SetPlayRate _skeletalmesh_3 1.0)
        (Utilities|FlowControl|Delay (Math|Random|RandomFloatinRange 5.0 25.0))
        (CallFunction|FLEE)))))

(event Custom|SHOW
  (bind _skeletalmesh (Variables|Default|GetSkeletalMesh))
  (bind _skeletalmesh_2 (Variables|Default|GetSkeletalMesh))
  ;[1 0.2527 0.8639] SHOW
  (if (not (Variables|Default|GetFrogFLEEING))
    (Utilities|FlowControl|Delay (Math|Random|RandomFloatinRange 1.0 3e+01))
    (Components|Animation|PlayAnimation _skeletalmesh "/Game/NotewatchContent/Creatures/Frog/Other/Jump.Jump" true)
    (Components|Timeline|SetPlayRate _skeletalmesh 2.0)
    (switch int (Math|Random|RandomIntegerinRange 0 2)
      (:0
        (Variables|Default|SetStartLOC (Variables|Default|GetLOC1))
        (Variables|Default|SetStartROT (Variables|Default|GetROT1)))
      (:1
        (Variables|Default|SetStartLOC (Variables|Default|GetLOC2))
        (Variables|Default|SetStartROT (Variables|Default|GetROT2)))
      (:2
        (Variables|Default|SetStartLOC (Variables|Default|GetLOC3))
        (Variables|Default|SetStartROT (Variables|Default|GetROT3))))
    (Transformation|SetActorLocationAndRotation (- (Variables|Default|GetStartLOC) "300.000000,10.000000,300.000000") (Math|Rotator|MakeRotator 9e+01 (.pitch (Variables|Default|GetStartROT)) (.yaw (Variables|Default|GetStartROT))) false true)
    ;;[0 0 0 0.5] Sound
    (Audio|PlaySoundatLocation (.OutItem (Utilities|Array|Random (Utilities|Array|MakeArray "/Game/NotewatchContent/Audio/Sounds/Rustle1.Rustle1" "/Game/NotewatchContent/Audio/Sounds/Rustle2.Rustle2" "/Game/NotewatchContent/Audio/Sounds/Rustle3.Rustle3"))) (Transformation|GetWorldLocation (Variables|Default|GetDefSceneRoot)) "0, 0, 0" (Math|Random|RandomFloatinRange 0.25 0.5) (Math|Random|RandomFloatinRange 1.75 2.0) 0.0 "/Game/NotewatchContent/Audio/Sounds/RinglingerAmbientAtten.RinglingerAmbientAtten" 0 0 0)
    (Components|MoveComponentTo (Variables|Default|GetDefSceneRoot) (- (Variables|Default|GetStartLOC) "0.000000,0.000000,-100.000000") (Variables|Default|GetStartROT) true false 0.5 true)
    (Components|MoveComponentTo (Variables|Default|GetDefSceneRoot) (Variables|Default|GetStartLOC) (Variables|Default|GetStartROT) false true 0.5 true)
    (Components|Animation|PlayAnimation _skeletalmesh_2 "/Game/NotewatchContent/Creatures/Frog/Other/Idle.Idle" true)
    (Components|Timeline|SetPlayRate _skeletalmesh_2 1.0)
    (Utilities|FlowControl|Delay (Math|Random|RandomFloatinRange 5.0 25.0))
    (CallFunction|FLEE)))

(event EventTick
  (params (DeltaSeconds :type Float%20%28single-precision%29))
  ;[0.132 1 0 0.5] RIBBIT
  (Utilities|FlowControl|Delay (Math|Random|RandomFloatinRange 0.0 1e+01))
  ;;[0 0 0 0.5] Sound
  (Audio|PlaySoundatLocation "/Game/NotewatchContent/Audio/Sounds/Frog.Frog" (Transformation|GetWorldLocation (Variables|Default|GetDefSceneRoot)) "0, 0, 0" (Math|Random|RandomFloatinRange 0.1 0.5) (Math|Random|RandomFloatinRange 0.5 2.0) 0.0 "/Game/NotewatchContent/Audio/Sounds/RinglingerAmbientAtten.RinglingerAmbientAtten" 0 0 0))

(fn ConstructionScript)