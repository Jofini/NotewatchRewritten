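; Ambient rabbit creature that flees with rustle sounds and Niagara effects, then reappears elsewhere.
; FLEE, after a short random delay, moves the sped-up animated mesh toward a point below the effect, then teleports it far below the world.
; After a random wait, it picks one of three stored spots and eases the mesh in from below, restoring normal animation speed.
; SHOW shares this reappearance path, guarded by BunnyFLEEING.
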(event Custom|FLEE
  (bind _skeletalmesh (Variables|Default|GetSkeletalMesh))
  (bind _skeletalmesh_2 (Variables|Default|GetSkeletalMesh))
  (bind _niagara (Variables|Default|GetNiagara))
  (bind _skeletalmesh_3 (Variables|Default|GetSkeletalMesh))
  (bind _returnvalue (Transformation|GetWorldRotation _niagara))
  (bind _returnvalue_2 (Transformation|GetWorldLocation _niagara))
  ;[0 0.2291 1] FLEE
  (Utilities|FlowControl|Delay (Math|Random|RandomFloatinRange 0.0 2.0))
  (Utilities|FlowControl|Sequence
    (:then_0
      (goto _label Stop))
    (:then_1
      (if (not (Variables|Default|GetBunnyFLEEING))
        (Variables|Default|SetBunnyFLEEING true)
        ;;[0 0 0 0.5] Sound
        (Audio|PlaySoundatLocation "/Game/NotewatchContent/Audio/Sounds/Brush.Brush" _returnvalue_2 "0, 0, 0" (Math|Random|RandomFloatinRange 1.0 1.0) (Math|Random|RandomFloatinRange 1.0 2.0) 0.0 "/Game/NotewatchContent/Audio/Sounds/RinglingerAmbientAtten.RinglingerAmbientAtten" 0 0 0)
        ;;[0 0 0 0.5] Sound
        (Audio|PlaySoundatLocation (.OutItem (Utilities|Array|Random (Utilities|Array|MakeArray "/Game/NotewatchContent/Audio/Sounds/Rustle1.Rustle1" "/Game/NotewatchContent/Audio/Sounds/Rustle2.Rustle2" "/Game/NotewatchContent/Audio/Sounds/Rustle3.Rustle3"))) _returnvalue_2 "0, 0, 0" (Math|Random|RandomFloatinRange 0.5 1.0) (Math|Random|RandomFloatinRange 1.0 2.0) 0.0 "/Game/NotewatchContent/Audio/Sounds/RinglingerAmbientAtten.RinglingerAmbientAtten" 0 0 0)
        (Components|Activation|Activate (Variables|Default|GetNiagara) true)
        (Components|Animation|PlayAnimation _skeletalmesh "/Game/NotewatchContent/Creatures/Rabbit/Other/Rabbit_Anim.Rabbit_Anim" true)
        (Components|Timeline|SetPlayRate _skeletalmesh 5.0)
        (Components|MoveComponentTo _skeletalmesh (- _returnvalue_2 "0.000000,0.000000,250.000000") (Math|Rotator|MakeRotator -1.2e+02 (.pitch _returnvalue) (.yaw _returnvalue)) true false 3.0 false)
        (Components|Activation|Deactivate (Variables|Default|GetNiagara))
        (Variables|Default|SetStartLOC "0.000000,0.000000,-50000.000000")
        (Transformation|SetWorldLocation (Variables|Default|GetSkeletalMesh) (Variables|Default|GetStartLOC) false true)
        (Transformation|SetActorLocation (Variables|Default|GetStartLOC) false true)
        (Utilities|FlowControl|Delay (Math|Random|RandomFloatinRange 1.0 6e+01))
        (Variables|Default|SetBunnyFLEEING false)
        ;[1 0.2527 0.8639] SHOW
        (Components|Animation|PlayAnimation _skeletalmesh_2 "/Game/NotewatchContent/Creatures/Rabbit/Other/Rabbit_Anim.Rabbit_Anim" true)
        (Components|Timeline|SetPlayRate _skeletalmesh_2 5.0)
        (switch int (Math|Random|RandomIntegerinRange 0 2)
          (:0
            (Variables|Default|SetStartLOC (Variables|Default|GetLOC1))
            (Variables|Default|SetStartROT (Variables|Default|GetROT1)))
          (:1
            (Variables|Default|SetStartLOC (Variables|Default|GetLOC2))
            (Variables|Default|SetStartROT (Variables|Default|GetROT2)))
          (:2
            (Variables|Default|SetStartLOC (Variables|Default|GetLOC3))
            (Variables|Default|SetStartROT (Variables|Default|GetROT3))))
        (Transformation|SetActorLocationAndRotation (- (Variables|Default|GetStartLOC) "0.000000,0.000000,500.000000") (Math|Random|RandomRotator false) false true)
        (Components|Activation|Activate (Variables|Default|GetNiagara) false)
        ;;[0 0 0 0.5] Sound
        (Audio|PlaySoundatLocation (.OutItem (Utilities|Array|Random (Utilities|Array|MakeArray "/Game/NotewatchContent/Audio/Sounds/Rustle1.Rustle1" "/Game/NotewatchContent/Audio/Sounds/Rustle2.Rustle2" "/Game/NotewatchContent/Audio/Sounds/Rustle3.Rustle3"))) (Transformation|GetWorldLocation (Variables|Default|GetSkeletalMesh)) "0, 0, 0" (Math|Random|RandomFloatinRange 0.25 0.5) (Math|Random|RandomFloatinRange 1.75 2.0) 0.0 "/Game/NotewatchContent/Audio/Sounds/RinglingerAmbientAtten.RinglingerAmbientAtten" 0 0 0)
        (Components|MoveComponentTo _skeletalmesh_3 (Variables|Default|GetStartLOC) (Variables|Default|GetStartROT) true true 2.5 true :!label _label)
        (Components|Animation|PlayAnimation _skeletalmesh_3 "/Game/NotewatchContent/Creatures/Rabbit/Other/Rabbit_Anim.Rabbit_Anim" true)
        (Components|Timeline|SetPlayRate _skeletalmesh_3 1.0)
        (Components|Activation|Deactivate (Variables|Default|GetNiagara))))))

(event Custom|SHOW
  (bind _skeletalmesh (Variables|Default|GetSkeletalMesh))
  (bind _skeletalmesh_2 (Variables|Default|GetSkeletalMesh))
  ;[1 0.2527 0.8639] SHOW
  (if (not (Variables|Default|GetBunnyFLEEING))
    (Components|Activation|Deactivate (Variables|Default|GetNiagara))
    (Utilities|FlowControl|Delay (Math|Random|RandomFloatinRange 1.0 6e+01))
    (Components|Animation|PlayAnimation _skeletalmesh "/Game/NotewatchContent/Creatures/Rabbit/Other/Rabbit_Anim.Rabbit_Anim" true)
    (Components|Timeline|SetPlayRate _skeletalmesh 5.0)
    (switch int (Math|Random|RandomIntegerinRange 0 2)
      (:0
        (Variables|Default|SetStartLOC (Variables|Default|GetLOC1))
        (Variables|Default|SetStartROT (Variables|Default|GetROT1)))
      (:1
        (Variables|Default|SetStartLOC (Variables|Default|GetLOC2))
        (Variables|Default|SetStartROT (Variables|Default|GetROT2)))
      (:2
        (Variables|Default|SetStartLOC (Variables|Default|GetLOC3))
        (Variables|Default|SetStartROT (Variables|Default|GetROT3))))
    (Transformation|SetActorLocationAndRotation (- (Variables|Default|GetStartLOC) "0.000000,0.000000,500.000000") (Math|Random|RandomRotator false) false true)
    (Components|Activation|Activate (Variables|Default|GetNiagara) false)
    ;;[0 0 0 0.5] Sound
    (Audio|PlaySoundatLocation (.OutItem (Utilities|Array|Random (Utilities|Array|MakeArray "/Game/NotewatchContent/Audio/Sounds/Rustle1.Rustle1" "/Game/NotewatchContent/Audio/Sounds/Rustle2.Rustle2" "/Game/NotewatchContent/Audio/Sounds/Rustle3.Rustle3"))) (Transformation|GetWorldLocation (Variables|Default|GetSkeletalMesh)) "0, 0, 0" (Math|Random|RandomFloatinRange 0.25 0.5) (Math|Random|RandomFloatinRange 1.75 2.0) 0.0 "/Game/NotewatchContent/Audio/Sounds/RinglingerAmbientAtten.RinglingerAmbientAtten" 0 0 0)
    (Components|MoveComponentTo _skeletalmesh_2 (Variables|Default|GetStartLOC) (Variables|Default|GetStartROT) true true 2.5 true)
    (Components|Animation|PlayAnimation _skeletalmesh_2 "/Game/NotewatchContent/Creatures/Rabbit/Other/Rabbit_Anim.Rabbit_Anim" true)
    (Components|Timeline|SetPlayRate _skeletalmesh_2 1.0)
    (Components|Activation|Deactivate (Variables|Default|GetNiagara))))

(fn ConstructionScript)