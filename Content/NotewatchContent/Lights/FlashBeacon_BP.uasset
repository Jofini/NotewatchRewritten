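; Player flashlight spotlight that follows the character's aim, fades in at begin play before enabling input, and flickers at random while on.
; The flash input triggers a fading intensity burst and a camera-forward line trace that ignores the player and certain plant actors.
; A chain of casts on the hit actor makes creatures flee, except Goldeer, which dies.
; When off, the light hides and flash input plays only a lower-pitched sound.
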(event Custom|Flicker
  ;[1 1 1 0.5] Flicker
  (if (Variables|Default|GetON)
    (if (Variables|Default|GetFLASH)
      (Rendering|SetActorHiddenInGame false)
      (else
        (Utilities|FlowControl|Delay (Math|Random|RandomFloatinRange 0.001 5.0))
        (Rendering|SetActorHiddenInGame true)
        (Utilities|FlowControl|Delay (Math|Random|RandomFloatinRange 0.001 0.5))
        (Rendering|SetActorHiddenInGame false)))))

(event Input|EnhancedActionEvents|EnhancedInputActionIA_Flash
  (params (ActionValue :type Boolean) (ElapsedSeconds :type Float%20%28double-precision%29) (TriggeredSeconds :type Float%20%28double-precision%29) (InputAction :type Input%20Action%20Object%20Reference :default "/Game/FirstPerson/Input/Actions/IA_Flash.IA_Flash"))
  (bind _returnvalue (Math|Random|RandomFloatinRange 0.9 1.1))
  ;[1 0.8314 0 0.502] Flash
  (if (Variables|Default|GetON)
    (Variables|Default|SetFLASH true)
    (Utilities|FlowControl|Sequence
      (:then_0
        (Audio|SpawnSound2D "/Game/NotewatchContent/Audio/Sounds/Flashlight.Flashlight" _returnvalue _returnvalue 0.1 0)
        (Rendering|Components|Light|SetIntensity (Variables|Default|GetSpotLightComponent) 2.5e+04)
        (bind _lightfadetl (Timeline|LightFade PlayFromStart)
          (:Update
            (Rendering|Components|Light|SetIntensity (Variables|Default|GetSpotLightComponent) _lightfadetl))
          (:Finished
            (Variables|Default|SetFLASH false))))
      (:then_1
        ;[0 0.2646 1 0.5] Line Tracing
        (bind _returnvalue_2 (Actor|GetActorOfClass "/Game/NotewatchContent/Monsters/Spicreep/BP/Spicreep_BP.Spicreep_BP_C"))
        (bind _returnvalue_3 (Actor|GetActorOfClass "/Game/NotewatchContent/Quests/AsterFlower/BP/AsterFlower_BP.AsterFlower_BP_C"))
        (bind _returnvalue_4 (Actor|GetActorOfClass "/Game/NotewatchContent/Quests/Chrysogonum/BP/Chrysogonum_BP.Chrysogonum_BP_C"))
        (bind _returnvalue_5 (Actor|GetActorOfClass "/Game/NotewatchContent/Quests/Amanita/BP/Amanita_BP.Amanita_BP_C"))
        (bind _returnvalue_6 (Actor|GetActorOfClass "/Game/NotewatchContent/Quests/CardinalFlower/BP/CardinalFlower_BP.CardinalFlower_BP_C"))
        (bind _returnvalue_7 (Actor|GetActorOfClass "/Game/NotewatchContent/Quests/SwampMilkweed/BP/SwampMilkweed_BP.SwampMilkweed_BP_C"))
        (bind _outhit (Collision|LineTraceByChannel (Transformation|GetWorldLocation (Variables|/Game/FirstPerson/Blueprints/BP_FirstPersonCharacter.BP_FirstPersonCharacter_C|GetFirstPersonCamera (stale EventTick _returnvalue))) (+ (Transformation|GetWorldLocation (Variables|/Game/FirstPerson/Blueprints/BP_FirstPersonCharacter.BP_FirstPersonCharacter_C|GetFirstPersonCamera (stale EventTick _returnvalue))) (* (Math|Vector|GetForwardVector (Variables|/Game/FirstPerson/Blueprints/BP_FirstPersonCharacter.BP_FirstPersonCharacter_C|GetFirstPersonCamera (stale EventTick _returnvalue))) (Variables|Components|GetEndPoint))) "TraceTypeQuery2" true (Utilities|Array|MakeArray (stale EventTick _returnvalue) _returnvalue_2 _returnvalue_3 _returnvalue_4 _returnvalue_5 _returnvalue_6 _returnvalue_7) "None"))
        (Utilities|FlowControl|Sequence
          (:then_0
            (bind _asringlinger_bp (Utilities|Casting|CastToRinglinger_BP (.HitActor (Collision|BreakHitResult _outhit))))
            (Default|FLEE _asringlinger_bp))
          (:then_1
            (bind _asroboach_bp (Utilities|Casting|CastToRoboach_BP (.HitActor (Collision|BreakHitResult _outhit))))
            (Default|FLEE _asroboach_bp))
          (:then_2
            (bind _asasset_bp (Utilities|Casting|CastToAsset_BP (.HitActor (Collision|BreakHitResult _outhit))))
            (Default|FLEE _asasset_bp))
          (:then_3
            (bind _asbaloon_bp (Utilities|Casting|CastToBaloon_BP (.HitActor (Collision|BreakHitResult _outhit))))
            (Default|FLEE _asbaloon_bp))
          (:then_4
            (bind _ashighpointer_bp (Utilities|Casting|CastToHighpointer_BP (.HitActor (Collision|BreakHitResult _outhit))))
            (Default|FLEE _ashighpointer_bp))
          (:then_5
            (bind _asleeth_bp (Utilities|Casting|CastToLeeth_BP (.HitActor (Collision|BreakHitResult _outhit))))
            (Default|FLEE _asleeth_bp))
          (:then_6
            (bind _asgoldeer_bp (Utilities|Casting|CastToGoldeer_BP (.HitActor (Collision|BreakHitResult _outhit))))
            (Default|DIE _asgoldeer_bp))
          (:then_7
            (bind _astree_eye_bp (Utilities|Casting|CastToTreeEye_BP (.HitActor (Collision|BreakHitResult _outhit))))
            (Default|FLEE _astree_eye_bp))
          (:then_8
            (bind _asdenten_bp (Utilities|Casting|CastToDenten_BP (.HitActor (Collision|BreakHitResult _outhit))))
            (Default|FLEE _asdenten_bp)))))
    (else
      ;;[1 0 0 0.5] OFF
      (Audio|SpawnSound2D "/Game/NotewatchContent/Audio/Sounds/Flashlight.Flashlight" _returnvalue (Math|Random|RandomFloatinRange 0.5 0.75) 0.1 0))))

(event EventBeginPlay
  ;[0 1 0.1303 0.5] Enable Input
  (bind _nightlight (Timeline|Timeline PlayFromStart)
    (:Update
      (Rendering|Components|Light|SetIntensity (Variables|Default|GetSpotLightComponent) _nightlight))
    (:Finished
      (Input|EnableInput (Game|GetPlayerController 0))
      (Variables|Components|SetNightStartOVER true))))

(event EventTick
  (params (DeltaSeconds :type Float%20%28single-precision%29))
  ;[0.6769 0.2762 0.8281 0.5] Rotate With Camera
  (if (Variables|Default|GetON)
    (Utilities|FlowControl|Sequence
      (:then_0
        (bind _returnvalue (Actor|GetActorOfClass "/Game/FirstPerson/Blueprints/BP_FirstPersonCharacter.BP_FirstPersonCharacter_C"))
        (Transformation|SetActorRotation (Pawn|GetBaseAimRotation _returnvalue)))
      (:then_1
        (if (Variables|Components|GetNightStartOVER)
          (CallFunction|Flicker))))
    (else
      (Rendering|SetActorHiddenInGame true))))

(fn ConstructionScript)