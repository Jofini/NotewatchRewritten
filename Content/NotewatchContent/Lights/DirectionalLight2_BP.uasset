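; Directional light Blueprint that varies its intensity over time as a night light.
; On BeginPlay a start timeline drives the light component's intensity and sets a flag when it finishes.
; Tick then replays a second timeline, NightLight, whenever it is not already running, so the intensity variation loops indefinitely.
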(event EventBeginPlay
  ;[0.15 0.15 0.15 0.5] NightLight Variance
  (bind _nightlight (Timeline|Timeline PlayFromStart)
    (:Update
      (Rendering|Components|Light|SetIntensity (Variables|Default|GetLightComponent) _nightlight))
    (:Finished
      (Variables|Default|SetNightStartOVER true))))

(event EventTick
  (params (DeltaSeconds :type Float%20%28single-precision%29))
  ;[0.15 0.15 0.15 0.5] NightLight Variance
  (if (Variables|Default|GetNightStartOVER)
    (if (not (Variables|Default|GetNightLightBEGIN))
      (Variables|Default|SetNightLightBEGIN true)
      (bind _nightlight (Timeline|NightLight PlayFromStart)
        (:Update
          (Rendering|Components|Light|SetIntensity (Variables|Default|GetLightComponent) _nightlight))
        (:Finished
          (Variables|Default|SetNightLightBEGIN false))))))

(fn ConstructionScript)