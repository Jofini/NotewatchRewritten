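; Amanita mushroom quest actor that plays a pickup effect and removes itself when its Collect event is called.
; Collect plays a random grass-pick sound and a brush sound with varied pitch, activates two Niagara effects, then eases the root upward with a spin using MoveComponentTo.
; When the move completes, it destroys the mushroom component, deactivates the effects and waits briefly before destroying the actor.
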(event Custom|Collect
  (bind _amanita (Variables|Default|GetAmanita))
  (bind _returnvalue (Transformation|GetWorldLocation _amanita))
  (Utilities|FlowControl|Sequence
    (:then_0
      (goto _label Stop))
    (:then_1
      ;[0 1 0.02625] Sound
      (Audio|PlaySoundatLocation (.OutItem (Utilities|Array|Random (Utilities|Array|MakeArray "/Game/NotewatchContent/Audio/Sounds/GrassPick1.GrassPick1" "/Game/NotewatchContent/Audio/Ambience/GrassPick2.GrassPick2" "/Game/NotewatchContent/Audio/Sounds/GrassPick3.GrassPick3" "/Game/NotewatchContent/Audio/Sounds/GrassPick4.GrassPick4" "/Game/NotewatchContent/Audio/Sounds/GrassPick5.GrassPick5"))) _returnvalue "0, 0, 0" (Math|Random|RandomFloatinRange 3.0 3.0) (Math|Random|RandomFloatinRange 0.75 1.25) 0.0 0 0 0 0)
      ;[0 1 0.02625] Sound
      (Audio|PlaySoundatLocation "/Game/NotewatchContent/Audio/Sounds/Brush.Brush" _returnvalue "0, 0, 0" (Math|Random|RandomFloatinRange 1.0 1.0) (Math|Random|RandomFloatinRange 1.0 1.5) 0.0 0 0 0 0)
      (Components|Activation|Activate (Variables|Default|GetNiagara1) true)
      (Components|MoveComponentTo (Variables|Default|GetDefaultSceneRoot) (+ _returnvalue "0.000000,0.000000,100.000000") "0.000000,1000.000000,0.000000" true true 0.5 false :!label _label)
      (Components|DestroyComponent (Variables|Default|GetAmanita))
      (Components|Activation|Deactivate (Variables|Default|GetNiagara))
      (Utilities|FlowControl|Delay 2.5)
      (Actor|DestroyActor))))

(event EventBeginPlay)

(event Collision|EventActorBeginOverlap
  (params (OtherActor :type Actor%20Object%20Reference)))

(event EventTick
  (params (DeltaSeconds :type Float%20%28single-precision%29)))

(fn ConstructionScript)