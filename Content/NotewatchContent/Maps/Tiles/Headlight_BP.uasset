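; Headlight prop that flickers at random, switching its spot light off and back on with sound.
; Tick runs a flicker cycle guarded by a LightFlicker flag, using random delays for both the lit and dark periods.
; Each switch plays a random, pitch-varied flicker sound at the point light's location, and the LightSound volume drops while the spot light is hidden.
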(event EventBeginPlay)

(event EventTick
  (params (DeltaSeconds :type Float%20%28single-precision%29))
  (if (not (Variables|Default|GetLightFlicker))
    (Variables|Default|SetLightFlicker true)
    (Utilities|FlowControl|Delay (Math|Random|RandomFloatinRange 0.1 5.0))
    ;[0 0 0 0.5] Sound
    (Audio|PlaySoundatLocation (.OutItem (Utilities|Array|Random (Utilities|Array|MakeArray "/Game/NotewatchContent/Audio/Sounds/Flicker1.Flicker1" "/Game/NotewatchContent/Audio/Sounds/Flicker2.Flicker2" "/Game/NotewatchContent/Audio/Sounds/Flicker3.Flicker3"))) (Transformation|GetWorldLocation (Variables|Default|GetPointLightComponent)) "0, 0, 0" 0.5 (Math|Random|RandomFloatinRange 0.5 0.75) 0.0 "/Game/NotewatchContent/Audio/Sounds/RinglingerAmbientAtten.RinglingerAmbientAtten" 0 0 0)
    (Audio|Components|Audio|SetVolumeMultiplier (Variables|Default|GetLightSound) 0.25 :!class /Script/Engine.AudioComponent)
    (Development|SetHiddeninGame (Variables|Default|GetSpotLightComponent) true false)
    (Utilities|FlowControl|Delay (Math|Random|RandomFloatinRange 0.1 1.0))
    (Development|SetHiddeninGame (Variables|Default|GetSpotLightComponent) false false)
    (Audio|Components|Audio|SetVolumeMultiplier (Variables|Default|GetLightSound) 0.75 :!class /Script/Engine.AudioComponent)
    (Variables|Default|SetLightFlicker false)
    ;[0 0 0 0.5] Sound
    (Audio|PlaySoundatLocation (.OutItem (Utilities|Array|Random (Utilities|Array|MakeArray "/Game/NotewatchContent/Audio/Sounds/Flicker1.Flicker1" "/Game/NotewatchContent/Audio/Sounds/Flicker2.Flicker2" "/Game/NotewatchContent/Audio/Sounds/Flicker3.Flicker3"))) (Transformation|GetWorldLocation (Variables|Default|GetPointLightComponent)) "0, 0, 0" 0.5 (Math|Random|RandomFloatinRange 0.5 0.75) 0.0 "/Game/NotewatchContent/Audio/Sounds/RinglingerAmbientAtten.RinglingerAmbientAtten" 0 0 0)))

(fn ConstructionScript)