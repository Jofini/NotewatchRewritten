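; Highpointer is a monster that slowly descends onto one of three random locations and kills the player if not driven off in time.
; HUNT starts the cycle after a long random delay; once a descent completes, a countdown leads to DIE, which turns and freezes the player, then lunges at the camera.
; FLEE halts the descent, launches it skyward, hides it far below and restarts after a cooldown, with HPINVIN and HPKILL flags gating both outcomes.
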(event Custom|FLEE
  (bind _returnvalue (Math|Random|RandomFloatinRange -2.5e+03 2.5e+03))
  (bind _returnvalue_2 (Math|Random|RandomRotator true))
  (bind _returnvalue_3 (Math|Random|RandomRotator true))
  (bind _skeletalmesh (Variables|Default|GetSkeletalMesh))
  (bind _skeletalmesh_2 (Variables|Default|GetSkeletalMesh))
  (bind _defaultsceneroot (Variables|Default|GetDefaultSceneRoot))
  ;[0 0.2291 1] FLEE
  (Utilities|FlowControl|Sequence
    (:then_0
      (goto _label Stop))
    (:then_1
      (if (not (Variables|Default|GetHPINVIN))
        (Variables|Default|SetHPINVIN true)
        (Variables|Default|SetHPKILL false)
        ;;[0 0 0 0.5] Sound
        (Audio|PlaySoundatLocation (.OutItem (Utilities|Array|Random (Utilities|Array|MakeArray "/Game/NotewatchContent/Audio/Sounds/HighPointer1.HighPointer1" "/Game/NotewatchContent/Audio/Sounds/HighPointer2.HighPointer2" "/Game/NotewatchContent/Audio/Sounds/HighPointer3.HighPointer3"))) "0, 0, 0" "0, 0, 0" (Math|Random|RandomFloatinRange 0.05 0.5) (Math|Random|RandomFloatinRange 0.5 1.5) 0.0 0 0 0 0)
        (Components|Animation|PlayAnimation _skeletalmesh "/Game/NotewatchContent/Monsters/Highpointer/Other/HighPointer_Anim.HighPointer_Anim" true)
        (Components|Timeline|SetPlayRate _skeletalmesh 1.0)
        (Components|MoveComponentTo _defaultsceneroot (+ (Variables|Default|GetStartLOC) (Math|Vector|MakeVector _returnvalue _returnvalue 2e+03)) _returnvalue_3 false true 1.0 true)
        (Components|MoveComponentTo _defaultsceneroot (+ (Variables|Default|GetStartLOC) (Math|Vector|MakeVector _returnvalue _returnvalue 1e+05)) _returnvalue_3 false true 5.0 true)
        (Variables|Default|SetStartLOC "0.000000,0.000000,-50000.000000")
        (Transformation|SetWorldLocation (Variables|Default|GetDefaultSceneRoot) (Variables|Default|GetStartLOC) false true)
        (Transformation|SetActorLocation (Variables|Default|GetStartLOC) false true)
        (Utilities|FlowControl|Delay (Math|Random|RandomFloatinRange 2e+01 4e+01))
        (Variables|Default|SetHPINVIN false)
        (Variables|Default|SetHPKILL false)
        ;[1 0.2527 0.8639] HUNT
        (Components|Animation|PlayAnimation _skeletalmesh_2 "/Game/NotewatchContent/Monsters/Highpointer/Other/HighPointer_Anim.HighPointer_Anim" true)
        (Components|Timeline|SetPlayRate _skeletalmesh_2 0.25)
        (switch int (Math|Random|RandomIntegerinRange 0 2)
          (:0
            (Variables|Default|SetStartLOC (Variables|Default|GetLOC1)))
          (:1
            (Variables|Default|SetStartLOC (Variables|Default|GetLOC2)))
          (:2
            (Variables|Default|SetStartLOC (Variables|Default|GetLOC3))))
        (Transformation|SetActorLocationAndRotation (+ (Variables|Default|GetStartLOC) "0.000000,0.000000,10000.000000") _returnvalue_2 false true)
        (Transformation|SetWorldRotation (Variables|Actor|GetStaticMesh) _returnvalue_2 false true)
        (Transformation|SetWorldLocation (Variables|Default|GetDefaultSceneRoot) (Transformation|GetActorLocation) false true)
        (Utilities|FlowControl|Delay 1.0)
        (Components|MoveComponentTo (Variables|Default|GetDefaultSceneRoot) (Variables|Default|GetStartLOC) _returnvalue_2 true false (Math|Random|RandomFloatinRange 35.0 45.0) false :!label _label)
        (Variables|Default|SetHPKILL true)
        (Utilities|FlowControl|RetriggerableDelay (Math|Random|RandomFloatinRange 3e+01 3e+01))
        (if (not (Variables|Default|GetHPINVIN))
          (if (Variables|Default|GetHPKILL)
            (CallFunction|DIE)))))))

(event Custom|HUNT
  (bind _returnvalue (Math|Random|RandomRotator true))
  (bind _skeletalmesh (Variables|Default|GetSkeletalMesh))
  ;[1 0.2527 0.8639] HUNT
  (Utilities|FlowControl|Delay (Math|Random|RandomFloatinRange 3e+02 6e+02))
  (Components|Animation|PlayAnimation _skeletalmesh "/Game/NotewatchContent/Monsters/Highpointer/Other/HighPointer_Anim.HighPointer_Anim" true)
  (Components|Timeline|SetPlayRate _skeletalmesh 0.25)
  (switch int (Math|Random|RandomIntegerinRange 0 2)
    (:0
      (Variables|Default|SetStartLOC (Variables|Default|GetLOC1)))
    (:1
      (Variables|Default|SetStartLOC (Variables|Default|GetLOC2)))
    (:2
      (Variables|Default|SetStartLOC (Variables|Default|GetLOC3))))
  (Transformation|SetActorLocationAndRotation (+ (Variables|Default|GetStartLOC) "0.000000,0.000000,10000.000000") _returnvalue false true)
  (Transformation|SetWorldRotation (Variables|Actor|GetStaticMesh) _returnvalue false true)
  (Transformation|SetWorldLocation (Variables|Default|GetDefaultSceneRoot) (Transformation|GetActorLocation) false true)
  (Utilities|FlowControl|Delay 1.0)
  (Components|MoveComponentTo (Variables|Default|GetDefaultSceneRoot) (Variables|Default|GetStartLOC) _returnvalue true false (Math|Random|RandomFloatinRange 35.0 45.0) false)
  (Variables|Default|SetHPKILL true)
  (Utilities|FlowControl|RetriggerableDelay (Math|Random|RandomFloatinRange 3e+01 3e+01))
  (if (not (Variables|Default|GetHPINVIN))
    (if (Variables|Default|GetHPKILL)
      (CallFunction|DIE))))

(event Custom|DIE
  ;[1 0 0.005053] Comment
  (Variables|Default|SetHPINVIN true)
  (bind _returnvalue (Actor|GetActorOfClass "/Game/FirstPerson/Blueprints/BP_FirstPersonCharacter.BP_FirstPersonCharacter_C"))
  (Pawn|SetControlRotation (Game|GetPlayerController (Variables|/Script/Engine.Pawn|GetPlayerState _returnvalue)) (Math|Rotator|FindLookatRotation (Transformation|GetWorldLocation (Variables|/Game/FirstPerson/Blueprints/BP_FirstPersonCharacter.BP_FirstPersonCharacter_C|GetFirstPersonCamera _returnvalue)) (Transformation|GetWorldLocation (Variables|Default|GetDefaultSceneRoot))))
  (Pawn|Components|CharacterMovement|DisableMovement (Variables|/Script/Engine.Character|GetCharacterMovement _returnvalue))
  ;;[0 0 0 0.5] Sound
  (Audio|PlaySoundatLocation (.OutItem (Utilities|Array|Random (Utilities|Array|MakeArray "/Game/NotewatchContent/Audio/Sounds/HighPointer1.HighPointer1" "/Game/NotewatchContent/Audio/Sounds/HighPointer2.HighPointer2" "/Game/NotewatchContent/Audio/Sounds/HighPointer3.HighPointer3"))) (Transformation|GetWorldLocation (Variables|/Game/FirstPerson/Blueprints/BP_FirstPersonCharacter.BP_FirstPersonCharacter_C|GetFirstPersonCamera _returnvalue)) "0, 0, 0" (Math|Random|RandomFloatinRange 1.5 1.5) (Math|Random|RandomFloatinRange 1.25 1.5) 0.0 0 0 0 0)
  (Components|MoveComponentTo (Variables|Default|GetDefaultSceneRoot) (Transformation|GetWorldLocation (Variables|/Game/FirstPerson/Blueprints/BP_FirstPersonCharacter.BP_FirstPersonCharacter_C|GetFirstPersonCamera _returnvalue)) (Math|Random|RandomRotator true) false false 0.5 true)
  (Default|DIE _returnvalue))

(fn ConstructionScript)