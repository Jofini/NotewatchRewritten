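; Spicreep monster that rises at one of three random spots and creeps toward the player while unwatched, freezing when looked at.
; External LOOK/NOTLOOK events stop or restart its MoveComponentTo approach, and HUNT schedules a delayed spawn.
; Repeated FLEE calls build a counter until it retreats underground with rustling and Niagara effects, then respawns.
; Kill capsule overlap turns the player's view toward it, lunges at the camera and triggers player death.
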(event OnComponentBeginOverlap(KillCapsule)
  (params (OverlappedComponent :type Primitive%20Component%20Object%20Reference) (OtherActor :type Actor%20Object%20Reference) (OtherComp :type Primitive%20Component%20Object%20Reference) (OtherBodyIndex :type Integer) (bFromSweep :type Boolean) (SweepResult :type Hit%20Result%20Structure%20%28by%20ref%29))
  ;[1 0 0.005053] Comment
  (bind _returnvalue (Actor|GetActorOfClass "/Game/FirstPerson/Blueprints/BP_FirstPersonCharacter.BP_FirstPersonCharacter_C"))
  (if (== OtherActor _returnvalue)
    (CallFunction|DIE)))

(event Custom|FLEE
  (bind _returnvalue (Math|Random|RandomFloatinRange 0.25 0.5))
  (bind _skeletalmesh (Variables|Default|GetSkeletalMesh))
  (bind _defaultsceneroot (Variables|Default|GetDefaultSceneRoot))
  (bind _defaultsceneroot_2 (Variables|Default|GetDefaultSceneRoot))
  (bind _skeletalmesh_2 (Variables|Default|GetSkeletalMesh))
  (bind _returnvalue_2 (Transformation|GetWorldLocation _defaultsceneroot))
  ;[0 0.2291 1] FLEE
  (Utilities|FlowControl|Sequence
    (:then_0
      (if (not (Variables|Default|GetSPCFLEEING))
        (Variables|Default|SetFLEEInterval (+ (Variables|Default|GetFLEEInterval) (Math|Random|RandomIntegerinRange 1 3)))))
    (:then_1
      (if (> (Variables|Default|GetFLEEInterval) 30)
        (if (not (Variables|Default|GetSPCFLEEING))
          (Variables|Default|SetSPCFLEEING true)
          (Variables|Default|SetSPCKILL false)
          ;;[0 0 0 0.5] Sound
          (Audio|PlaySoundatLocation (.OutItem (Utilities|Array|Random (Utilities|Array|MakeArray "/Game/NotewatchContent/Audio/Sounds/Rustle1.Rustle1" "/Game/NotewatchContent/Audio/Sounds/Rustle2.Rustle2" "/Game/NotewatchContent/Audio/Sounds/Rustle3.Rustle3"))) _returnvalue_2 "0, 0, 0" (Math|Random|RandomFloatinRange 1.0 1.0) (Math|Random|RandomFloatinRange 0.5 1.5) 0.0 "/Game/NotewatchContent/Audio/Sounds/RinglingerAmbientAtten.RinglingerAmbientAtten" 0 0 0)
          ;;[0 0 0 0.5] Sound
          (Audio|PlaySoundatLocation "/Game/NotewatchContent/Audio/Sounds/Brush.Brush" _returnvalue_2 "0, 0, 0" (Math|Random|RandomFloatinRange 1.0 1.25) (Math|Random|RandomFloatinRange 0.75 1.25) 0.0 "/Game/NotewatchContent/Audio/Sounds/RinglingerAmbientAtten.RinglingerAmbientAtten" 0 0 0)
          (Components|Activation|Activate (Variables|Default|GetNiagara) true)
          (Components|Animation|PlayAnimation _skeletalmesh "/Game/NotewatchContent/Monsters/Spicreep/Other/Spicreep_Anim.Spicreep_Anim" true)
          (Components|Timeline|SetPlayRate _skeletalmesh 1.0)
          (Utilities|FlowControl|Sequence
            (:then_0
              (goto _label Stop))
            (:then_1
              (Components|MoveComponentTo _defaultsceneroot (Math|Interpolation|Ease "EaseOut" 1.0 _returnvalue_2 (+ (Variables|Default|GetStartLOC) "0.000000,0.000000,-100.000000") 5.0) (Variables|Default|GetStartROT) true false 1.0 true)
              (Components|MoveComponentTo (Variables|Default|GetDefaultSceneRoot) (+ (Variables|Default|GetStartLOC) "0.000000,0.000000,-500.000000") (Transformation|GetWorldRotation (Variables|Default|GetDefaultSceneRoot)) false false 3.0 true)
              (Variables|Default|SetFLEEInterval 0)
              (Utilities|FlowControl|Delay (Math|Random|RandomFloatinRange 1.0 1e+01))
              (Variables|Default|SetStartLOC "0.000000,0.000000,-50000.000000")
              (Transformation|SetWorldLocation _defaultsceneroot (Variables|Default|GetStartLOC) false true)
              (Transformation|SetActorLocation (Variables|Default|GetStartLOC) false true)
              (Variables|Default|SetSPCFLEEING false)
              (Components|Activation|Deactivate (Variables|Default|GetNiagara))
              ;[1 0.2527 0.8639] HUNT
              (Components|Animation|PlayAnimation _skeletalmesh_2 "/Game/NotewatchContent/Monsters/Spicreep/Other/Spicreep_Anim.Spicreep_Anim" true)
              (Components|Timeline|SetPlayRate _skeletalmesh_2 0.1)
              (Components|Activation|Activate (Variables|Default|GetNiagara) true)
              (switch int (Math|Random|RandomIntegerinRange 0 2)
                (:0
                  (Variables|Default|SetStartLOC (Variables|Default|GetLOC1))
                  (Variables|Default|SetStartROT (Variables|Default|GetROT1)))
                (:1
                  (Variables|Default|SetStartLOC (Variables|Default|GetLOC2))
                  (Variables|Default|SetStartROT (Variables|Default|GetROT2)))
                (:2
                  (Variables|Default|SetStartLOC (Variables|Default|GetLOC3))
                  (Variables|Default|SetStartROT (Variables|Default|GetROT3))))
              (Transformation|SetActorLocationAndRotation (+ (Variables|Default|GetStartLOC) "0.000000,0.000000,-500.000000") (Variables|Default|GetStartROT) false true)
              (Transformation|SetWorldLocationAndRotation _defaultsceneroot_2 (Variables|Default|GetStartLOC) (Variables|Default|GetStartROT) false true)
              (Audio|PlaySoundatLocation "/Game/NotewatchContent/Audio/Sounds/Brush.Brush" _returnvalue_2 "0, 0, 0" (Math|Random|RandomFloatinRange 0.5 0.75) (Math|Random|RandomFloatinRange 0.25 0.5) 0.0 "/Game/NotewatchContent/Audio/Sounds/RinglingerAmbientAtten.RinglingerAmbientAtten" 0 0 0)
              ;;[0 0 0 0.5] Sound
              (Audio|PlaySoundatLocation (.OutItem (Utilities|Array|Random (Utilities|Array|MakeArray "/Game/NotewatchContent/Audio/Sounds/Rustle1.Rustle1" "/Game/NotewatchContent/Audio/Sounds/Rustle2.Rustle2" "/Game/NotewatchContent/Audio/Sounds/Rustle3.Rustle3"))) _returnvalue_2 "0, 0, 0" _returnvalue _returnvalue 0.0 "/Game/NotewatchContent/Audio/Sounds/RinglingerAmbientAtten.RinglingerAmbientAtten" 0 0 0)
              (Components|MoveComponentTo _defaultsceneroot_2 (Variables|Default|GetStartLOC) (Variables|Default|GetStartROT) true true (Math|Random|RandomFloatinRange 2.5 5.0) true)
              (Components|Activation|Deactivate (Variables|Default|GetNiagara))
              (Variables|Default|SetSPCMove true)
              (bind _returnvalue_3 (Actor|GetActorOfClass "/Game/FirstPerson/Blueprints/BP_FirstPersonCharacter.BP_FirstPersonCharacter_C"))
              (Components|MoveComponentTo (Variables|Default|GetDefaultSceneRoot) (Math|Interpolation|Ease "EaseIn" 5.0 _returnvalue_2 (- (Transformation|GetActorLocation _returnvalue_3) "0.000000,0.000000,100.000000") 1.0) (Variables|Default|GetStartROT) false false 2e+02 true :!label _label))))))))

(event Custom|HUNT
  (bind _returnvalue (Math|Random|RandomFloatinRange 0.25 0.5))
  (bind _defaultsceneroot (Variables|Default|GetDefaultSceneRoot))
  (bind _defaultsceneroot_2 (Variables|Default|GetDefaultSceneRoot))
  (bind _skeletalmesh (Variables|Default|GetSkeletalMesh))
  (bind _returnvalue_2 (Transformation|GetWorldLocation _defaultsceneroot))
  ;[1 0.2527 0.8639] HUNT
  (if (not (Variables|Default|GetSPCFLEEING))
    (Utilities|FlowControl|Sequence
      (:then_0
        (goto _label Stop))
      (:then_1
        (goto _label_2 Stop))
      (:then_2
        ;[0 0.2291 1] FLEE
        (Components|MoveComponentTo _defaultsceneroot (Math|Interpolation|Ease "EaseOut" 1.0 _returnvalue_2 (+ (Variables|Default|GetStartLOC) "0.000000,0.000000,-100.000000") 5.0) (Variables|Default|GetStartROT) true false 1.0 true) ; enters at Stop
      )
      (:then_3
        (Components|MoveComponentTo (Variables|Default|GetDefaultSceneRoot) (+ (Variables|Default|GetStartLOC) "0.000000,0.000000,-500.000000") (Transformation|GetWorldRotation (Variables|Default|GetDefaultSceneRoot)) false false 3.0 true) ; enters at Stop
      )
      (:then_4
        (Utilities|FlowControl|Delay (Math|Random|RandomFloatinRange 35.0 7e+01))
        (Components|Animation|PlayAnimation _skeletalmesh "/Game/NotewatchContent/Monsters/Spicreep/Other/Spicreep_Anim.Spicreep_Anim" true)
        (Components|Timeline|SetPlayRate _skeletalmesh 0.1)
        (Components|Activation|Activate (Variables|Default|GetNiagara) true)
        (switch int (Math|Random|RandomIntegerinRange 0 2)
          (:0
            (Variables|Default|SetStartLOC (Variables|Default|GetLOC1))
            (Variables|Default|SetStartROT (Variables|Default|GetROT1)))
          (:1
            (Variables|Default|SetStartLOC (Variables|Default|GetLOC2))
            (Variables|Default|SetStartROT (Variables|Default|GetROT2)))
          (:2
            (Variables|Default|SetStartLOC (Variables|Default|GetLOC3))
            (Variables|Default|SetStartROT (Variables|Default|GetROT3))))
        (Transformation|SetActorLocationAndRotation (+ (Variables|Default|GetStartLOC) "0.000000,0.000000,-500.000000") (Variables|Default|GetStartROT) false true)
        (Transformation|SetWorldLocationAndRotation _defaultsceneroot_2 (Variables|Default|GetStartLOC) (Variables|Default|GetStartROT) false true)
        (Audio|PlaySoundatLocation "/Game/NotewatchContent/Audio/Sounds/Brush.Brush" _returnvalue_2 "0, 0, 0" (Math|Random|RandomFloatinRange 0.5 0.75) (Math|Random|RandomFloatinRange 0.25 0.5) 0.0 "/Game/NotewatchContent/Audio/Sounds/RinglingerAmbientAtten.RinglingerAmbientAtten" 0 0 0)
        ;;[0 0 0 0.5] Sound
        (Audio|PlaySoundatLocation (.OutItem (Utilities|Array|Random (Utilities|Array|MakeArray "/Game/NotewatchContent/Audio/Sounds/Rustle1.Rustle1" "/Game/NotewatchContent/Audio/Sounds/Rustle2.Rustle2" "/Game/NotewatchContent/Audio/Sounds/Rustle3.Rustle3"))) _returnvalue_2 "0, 0, 0" _returnvalue _returnvalue 0.0 "/Game/NotewatchContent/Audio/Sounds/RinglingerAmbientAtten.RinglingerAmbientAtten" 0 0 0)
        (Components|MoveComponentTo _defaultsceneroot_2 (Variables|Default|GetStartLOC) (Variables|Default|GetStartROT) true true (Math|Random|RandomFloatinRange 2.5 5.0) true :!label _label)
        (Components|Activation|Deactivate (Variables|Default|GetNiagara))
        (Variables|Default|SetSPCMove true)
        (bind _returnvalue_3 (Actor|GetActorOfClass "/Game/FirstPerson/Blueprints/BP_FirstPersonCharacter.BP_FirstPersonCharacter_C"))
        (Components|MoveComponentTo (Variables|Default|GetDefaultSceneRoot) (Math|Interpolation|Ease "EaseIn" 5.0 _returnvalue_2 (- (Transformation|GetActorLocation _returnvalue_3) "0.000000,0.000000,100.000000") 1.0) (Variables|Default|GetStartROT) false false 2e+02 true :!label _label_2)))))

(event Custom|DIE
  (bind _returnvalue (Math|Random|RandomFloatinRange 1.5 1.5))
  (bind _defaultsceneroot (Variables|Default|GetDefaultSceneRoot))
  (bind _defaultsceneroot_2 (Variables|Default|GetDefaultSceneRoot))
  (bind _returnvalue_2 (Transformation|GetWorldLocation _defaultsceneroot))
  ;[1 0 0.005053] Comment
  (Pawn|SetControlRotation (Game|GetPlayerController (Variables|/Script/Engine.Pawn|GetPlayerState (stale OnComponentBeginOverlap(KillCapsule) _returnvalue))) (Math|Rotator|FindLookatRotation (Transformation|GetWorldLocation (Variables|/Game/FirstPerson/Blueprints/BP_FirstPersonCharacter.BP_FirstPersonCharacter_C|GetFirstPersonCamera (stale OnComponentBeginOverlap(KillCapsule) _returnvalue))) _returnvalue_2))
  (Pawn|Components|CharacterMovement|DisableMovement (Variables|/Script/Engine.Character|GetCharacterMovement (stale OnComponentBeginOverlap(KillCapsule) _returnvalue)))
  ;;[0 0 0 0.5] Sound
  (Audio|PlaySoundatLocation (.OutItem (Utilities|Array|Random (Utilities|Array|MakeArray "/Game/NotewatchContent/Audio/Sounds/Rustle1.Rustle1" "/Game/NotewatchContent/Audio/Sounds/Rustle2.Rustle2" "/Game/NotewatchContent/Audio/Sounds/Rustle3.Rustle3"))) (Transformation|GetWorldLocation (Variables|/Game/FirstPerson/Blueprints/BP_FirstPersonCharacter.BP_FirstPersonCharacter_C|GetFirstPersonCamera (stale OnComponentBeginOverlap(KillCapsule) _returnvalue))) "0, 0, 0" _returnvalue (Math|Random|RandomFloatinRange 0.75 1.0) 0.0 0 0 0 0)
  (Audio|PlaySoundatLocation "/Game/NotewatchContent/Audio/Sounds/SpicreepRoar.SpicreepRoar" _returnvalue_2 "0, 0, 0" _returnvalue 1.0 0.0 0 0 0 0)
  (Components|MoveComponentTo _defaultsceneroot_2 (- (Transformation|GetWorldLocation (Variables|/Game/FirstPerson/Blueprints/BP_FirstPersonCharacter.BP_FirstPersonCharacter_C|GetFirstPersonCamera (stale OnComponentBeginOverlap(KillCapsule) _returnvalue))) "0.000000,0.000000,100.000000") (Transformation|GetWorldRotation _defaultsceneroot_2) false false 0.75 false)
  (Default|DIE (stale OnComponentBeginOverlap(KillCapsule) _returnvalue)))

(event Custom|LOOK
  ;[1 0.2527 0.8639] HUNT
  (if (Variables|Default|GetSPCMove)
    (if (not (Variables|Default|GetSPCFLEEING))
      (Components|Timeline|SetPlayRate (Variables|Default|GetSkeletalMesh) 0.0)
      (Components|MoveComponentTo (Variables|Default|GetDefaultSceneRoot) (Math|Interpolation|Ease "EaseIn" 5.0 (Transformation|GetWorldLocation (Variables|Default|GetDefaultSceneRoot)) (- (Transformation|GetActorLocation (stale Custom|FLEE _returnvalue_3)) "0.000000,0.000000,100.000000") 1.0) (Variables|Default|GetStartROT) false false 2e+02 true) ; enters at Stop
    )))

(event Custom|NOT%20LOOK
  ;[1 0.2527 0.8639] HUNT
  (if (Variables|Default|GetSPCMove)
    (if (not (Variables|Default|GetSPCFLEEING))
      (Components|Timeline|SetPlayRate (Variables|Default|GetSkeletalMesh) 0.1)
      (bind _returnvalue (Actor|GetActorOfClass "/Game/FirstPerson/Blueprints/BP_FirstPersonCharacter.BP_FirstPersonCharacter_C"))
      (Components|MoveComponentTo (Variables|Default|GetDefaultSceneRoot) (Math|Interpolation|Ease "EaseIn" 5.0 (Transformation|GetWorldLocation (Variables|Default|GetDefaultSceneRoot)) (- (Transformation|GetActorLocation _returnvalue) "0.000000,0.000000,100.000000") 1.0) (Variables|Default|GetStartROT) false false 2e+02 true))))

(fn ConstructionScript)