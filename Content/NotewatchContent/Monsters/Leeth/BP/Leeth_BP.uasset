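; Leeth monster Blueprint that drops onto one of three random perches and kills the player if left there too long.
; HUNT delays the first descent; arrival arms LeethKILL and a 30-second timer leading to DIE.
; FLEE cancels the attack, leaps away with sound and Niagara effects, hides below the world, then respawns.
; DIE, despite its name, jumpscares the player, forcing the view and freezing movement before killing them.
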(event Custom|FLEE
  (bind _returnvalue (Math|Random|RandomFloatinRange 0.0 0.1))
  (bind _returnvalue_2 (Math|Random|RandomFloatinRange 1.25 1.5))
  (bind _returnvalue_3 (Math|Random|RandomFloatinRange 0.5 1.0))
  (bind _skeletalmesh (Variables|Default|GetSkeletalMesh))
  (bind _niagara (Variables|Default|GetNiagara))
  (bind _defaultsceneroot (Variables|Default|GetDefaultSceneRoot))
  (bind _skeletalmesh_2 (Variables|Default|GetSkeletalMesh))
  (bind _defaultsceneroot_2 (Variables|Default|GetDefaultSceneRoot))
  (bind _returnvalue_4 (Transformation|GetWorldLocation _defaultsceneroot))
  ;[0 0.2291 1] FLEE
  (Utilities|FlowControl|Sequence
    (:then_0
      (goto _label Stop))
    (:then_1
      (if (not (Variables|Default|GetLeethINVIN))
        (Variables|Default|SetLeethINVIN true)
        (Variables|Default|SetLeethKILL false)
        ;;[0 0 0 0.5] Sound
        (Audio|PlaySoundatLocation (.OutItem (Utilities|Array|Random (Utilities|Array|MakeArray "/Game/NotewatchContent/Audio/Sounds/Leeth1.Leeth1" "/Game/NotewatchContent/Audio/Sounds/Leeth2.Leeth2" "/Game/NotewatchContent/Audio/Sounds/Leeth3.Leeth3"))) _returnvalue_4 "0, 0, 0" (Math|Random|RandomFloatinRange 0.5 1.0) (Math|Random|RandomFloatinRange 0.5 1.5) 0.0 0 0 0 0)
        ;;[0 0 0 0.5] Sound
        (Audio|PlaySoundatLocation "/Game/NotewatchContent/Audio/Ambience/GrassPick5.GrassPick5" _returnvalue_4 "0, 0, 0" _returnvalue_2 _returnvalue_3 0.0 "/Game/NotewatchContent/Audio/Sounds/RinglingerAmbientAtten.RinglingerAmbientAtten" 0 0 0)
        (Audio|PlaySoundatLocation "/Game/NotewatchContent/Audio/Sounds/GrassPick2.GrassPick2" _returnvalue_4 "0, 0, 0" _returnvalue_2 _returnvalue_3 0.0 "/Game/NotewatchContent/Audio/Sounds/RinglingerAmbientAtten.RinglingerAmbientAtten" 0 0 0)
        (Audio|PlaySoundatLocation "/Game/NotewatchContent/Audio/Sounds/Brush.Brush" _returnvalue_4 "0, 0, 0" _returnvalue_2 _returnvalue_3 0.0 "/Game/NotewatchContent/Audio/Sounds/RinglingerAmbientAtten.RinglingerAmbientAtten" 0 0 0)
        (Components|Activation|Activate (Variables|Default|GetNiagara) true)
        (Components|Animation|PlayAnimation _skeletalmesh "/Game/NotewatchContent/Monsters/Leeth/Other/Leap.Leap" true)
        (Components|Timeline|SetPlayRate _skeletalmesh 0.5)
        (Components|MoveComponentTo _defaultsceneroot (+ (Variables|Default|GetStartLOC) "1000.000000,30000.000000,4000.000000") (Transformation|GetWorldRotation _defaultsceneroot) false true 4.0 true)
        (Utilities|FlowControl|Delay 1.0)
        (Variables|Default|SetStartLOC "0.000000,0.000000,-50000.000000")
        (Transformation|SetWorldLocation _defaultsceneroot (Variables|Default|GetStartLOC) false true)
        (Transformation|SetActorLocation (Variables|Default|GetStartLOC) false true)
        (Utilities|FlowControl|Delay (Math|Random|RandomFloatinRange 1e+01 2e+01))
        (Variables|Default|SetLeethINVIN false)
        (Variables|Default|SetLeethKILL false)
        (Components|Activation|Deactivate (Variables|Default|GetNiagara))
        ;[1 0.2527 0.8639] HUNT
        (Components|Animation|PlayAnimation _skeletalmesh_2 "/Game/NotewatchContent/Monsters/Leeth/Other/Idle.Idle" true)
        (Components|Timeline|SetPlayRate _skeletalmesh_2 0.1)
        (switch int (Math|Random|RandomIntegerinRange 0 2)
          (:0
            (Variables|Default|SetStartLOC (Variables|Default|GetLOC1))
            (Variables|Default|SetStartROT (Variables|Default|GetROT1)))
          (:1
            (Variables|Default|SetStartLOC (Variables|Default|GetLOC2))
            (Variables|Default|SetStartROT (Variables|Default|GetROT2)))
          (:2
            (Variables|Default|SetStartLOC (Variables|Default|GetLOC3))
            (Variables|Default|SetStartROT (Variables|Default|GetROT3))))
        (Transformation|SetActorLocationAndRotation (+ (Variables|Default|GetStartLOC) "0.000000,0.000000,10000.000000") (Math|Random|RandomRotator false) false true)
        (Transformation|SetWorldRotation _defaultsceneroot_2 "0.000000,0.000000,90.000000" false false)
        (Transformation|SetWorldLocation _defaultsceneroot_2 (+ (Variables|Default|GetStartLOC) "0.000000,0.000000,10000.000000") false true)
        (Audio|PlaySoundatLocation "/Game/NotewatchContent/Audio/Ambience/GrassPick3.GrassPick3" _returnvalue_4 "0, 0, 0" (Math|Random|RandomFloatinRange 0.0 0.1) (Math|Random|RandomFloatinRange 0.5 0.75) 0.0 "/Game/NotewatchContent/Audio/Sounds/RinglingerAmbientAtten.RinglingerAmbientAtten" 0 0 0)
        (Components|Activation|Activate _niagara true)
        ;;[0 0 0 0.5] Sound
        (Audio|PlaySoundatLocation (.OutItem (Utilities|Array|Random (Utilities|Array|MakeArray "/Game/NotewatchContent/Audio/Sounds/Leeth1.Leeth1" "/Game/NotewatchContent/Audio/Sounds/Leeth2.Leeth2" "/Game/NotewatchContent/Audio/Sounds/Leeth3.Leeth3"))) _returnvalue_4 "0, 0, 0" _returnvalue _returnvalue 0.0 "/Game/NotewatchContent/Audio/Sounds/RinglingerAmbientAtten.RinglingerAmbientAtten" 0 0 0)
        (Components|MoveComponentTo _defaultsceneroot_2 (Variables|Default|GetStartLOC) (Variables|Default|GetStartROT) true true 1.0 true :!label _label)
        (Components|Activation|Deactivate _niagara)
        (Variables|Default|SetLeethKILL true)
        (Utilities|FlowControl|RetriggerableDelay (Math|Random|RandomFloatinRange 3e+01 3e+01))
        (if (Variables|Default|GetLeethKILL)
          (CallFunction|DIE))))))

(event Custom|HUNT
  (bind _returnvalue (Math|Random|RandomFloatinRange 0.0 0.1))
  (bind _niagara (Variables|Default|GetNiagara))
  (bind _defaultsceneroot (Variables|Default|GetDefaultSceneRoot))
  (bind _skeletalmesh (Variables|Default|GetSkeletalMesh))
  (bind _defaultsceneroot_2 (Variables|Default|GetDefaultSceneRoot))
  (bind _returnvalue_2 (Transformation|GetWorldLocation _defaultsceneroot))
  ;[1 0.2527 0.8639] HUNT
  (if (not (Variables|Default|GetLeethINVIN))
    (Utilities|FlowControl|Delay (Math|Random|RandomFloatinRange 1.5e+02 3e+02))
    (Components|Animation|PlayAnimation _skeletalmesh "/Game/NotewatchContent/Monsters/Leeth/Other/Idle.Idle" true)
    (Components|Timeline|SetPlayRate _skeletalmesh 0.1)
    (switch int (Math|Random|RandomIntegerinRange 0 2)
      (:0
        (Variables|Default|SetStartLOC (Variables|Default|GetLOC1))
        (Variables|Default|SetStartROT (Variables|Default|GetROT1)))
      (:1
        (Variables|Default|SetStartLOC (Variables|Default|GetLOC2))
        (Variables|Default|SetStartROT (Variables|Default|GetROT2)))
      (:2
        (Variables|Default|SetStartLOC (Variables|Default|GetLOC3))
        (Variables|Default|SetStartROT (Variables|Default|GetROT3))))
    (Transformation|SetActorLocationAndRotation (+ (Variables|Default|GetStartLOC) "0.000000,0.000000,10000.000000") (Math|Random|RandomRotator false) false true)
    (Transformation|SetWorldRotation _defaultsceneroot_2 "0.000000,0.000000,90.000000" false false)
    (Transformation|SetWorldLocation _defaultsceneroot_2 (+ (Variables|Default|GetStartLOC) "0.000000,0.000000,10000.000000") false true)
    (Audio|PlaySoundatLocation "/Game/NotewatchContent/Audio/Ambience/GrassPick3.GrassPick3" _returnvalue_2 "0, 0, 0" (Math|Random|RandomFloatinRange 0.0 0.1) (Math|Random|RandomFloatinRange 0.5 0.75) 0.0 "/Game/NotewatchContent/Audio/Sounds/RinglingerAmbientAtten.RinglingerAmbientAtten" 0 0 0)
    (Components|Activation|Activate _niagara true)
    ;[0 0.2291 1] FLEE
    ;;[0 0 0 0.5] Sound
    (Audio|PlaySoundatLocation (.OutItem (Utilities|Array|Random (Utilities|Array|MakeArray "/Game/NotewatchContent/Audio/Sounds/Leeth1.Leeth1" "/Game/NotewatchContent/Audio/Sounds/Leeth2.Leeth2" "/Game/NotewatchContent/Audio/Sounds/Leeth3.Leeth3"))) _returnvalue_2 "0, 0, 0" _returnvalue _returnvalue 0.0 "/Game/NotewatchContent/Audio/Sounds/RinglingerAmbientAtten.RinglingerAmbientAtten" 0 0 0)
    (Components|MoveComponentTo _defaultsceneroot_2 (Variables|Default|GetStartLOC) (Variables|Default|GetStartROT) true true 1.0 true)
    (Components|Activation|Deactivate _niagara)
    (Variables|Default|SetLeethKILL true)
    (Utilities|FlowControl|RetriggerableDelay (Math|Random|RandomFloatinRange 3e+01 3e+01))
    (if (Variables|Default|GetLeethKILL)
      (CallFunction|DIE))))

(event Custom|DIE
  (bind _returnvalue (Math|Random|RandomFloatinRange 1.5 1.5))
  (bind _defaultsceneroot (Variables|Default|GetDefaultSceneRoot))
  (bind _defaultsceneroot_2 (Variables|Default|GetDefaultSceneRoot))
  (bind _returnvalue_2 (Transformation|GetWorldLocation _defaultsceneroot_2))
  ;[1 0 0.005053] Comment
  (Variables|Default|SetLeethINVIN true)
  (Components|Activation|Activate (Variables|Default|GetNiagara) true)
  (Components|Animation|PlayAnimation (Variables|Default|GetSkeletalMesh) "/Game/NotewatchContent/Monsters/Leeth/Other/Leap.Leap" false)
  (Components|MoveComponentTo (Variables|Default|GetDefaultSceneRoot) (Variables|Default|GetKillLOC) (Variables|Default|GetKillROT) false false 1.0 true)
  (Components|Activation|Deactivate (Variables|Default|GetNiagara))
  (Utilities|FlowControl|Delay (Math|Random|RandomFloatinRange 1.0 1e+01))
  (Components|Animation|PlayAnimation (Variables|Default|GetSkeletalMesh) "/Game/NotewatchContent/Monsters/Leeth/Other/Leap.Leap" false)
  (bind _returnvalue_3 (Actor|GetActorOfClass "/Game/FirstPerson/Blueprints/BP_FirstPersonCharacter.BP_FirstPersonCharacter_C"))
  (Components|Activation|Activate (Variables|Default|GetNiagara) true)
  (Pawn|SetControlRotation (Game|GetPlayerController (Variables|/Script/Engine.Pawn|GetPlayerState _returnvalue_3)) (Math|Rotator|FindLookatRotation (Transformation|GetWorldLocation (Variables|/Game/FirstPerson/Blueprints/BP_FirstPersonCharacter.BP_FirstPersonCharacter_C|GetFirstPersonCamera _returnvalue_3)) _returnvalue_2))
  (Pawn|Components|CharacterMovement|DisableMovement (Variables|/Script/Engine.Character|GetCharacterMovement _returnvalue_3))
  ;;[0 0 0 0.5] Sound
  (Audio|PlaySoundatLocation (.OutItem (Utilities|Array|Random (Utilities|Array|MakeArray "/Game/NotewatchContent/Audio/Sounds/Rustle1.Rustle1" "/Game/NotewatchContent/Audio/Sounds/Rustle2.Rustle2" "/Game/NotewatchContent/Audio/Sounds/Rustle3.Rustle3"))) (Transformation|GetWorldLocation (Variables|/Game/FirstPerson/Blueprints/BP_FirstPersonCharacter.BP_FirstPersonCharacter_C|GetFirstPersonCamera _returnvalue_3)) "0, 0, 0" _returnvalue (Math|Random|RandomFloatinRange 0.75 1.25) 0.0 0 0 0 0)
  (Audio|PlaySoundatLocation "/Game/NotewatchContent/Audio/Sounds/Leeth3.Leeth3" _returnvalue_2 "0, 0, 0" _returnvalue 1.5 0.0 0 0 0 0)
  (Audio|PlaySoundatLocation "/Game/NotewatchContent/Audio/Sounds/Leeth2.Leeth2" (Transformation|GetWorldLocation (Variables|/Game/FirstPerson/Blueprints/BP_FirstPersonCharacter.BP_FirstPersonCharacter_C|GetFirstPersonCamera _returnvalue_3)) "0, 0, 0" _returnvalue 2.0 0.0 0 0 0 0)
  (Components|MoveComponentTo _defaultsceneroot (- (Transformation|GetWorldLocation _defaultsceneroot) "0.000000,0.000000,5000.000000") (Transformation|GetWorldRotation _defaultsceneroot) false false 0.75 true)
  (Default|DIE _returnvalue_3))

(fn ConstructionScript)