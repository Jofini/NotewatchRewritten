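; Balloon monster that periodically descends on one of three preset spots and kills the player if not driven off in time.
; HUNT waits a random delay, then drops it from high above; once it arrives, a timer leads to DIE.
; FLEE halts the descent, flies it off in one of two directions, parks it below the map, then restarts the approach.
; DIE turns the player's view to the balloon, freezes movement, lunges and kills the player.
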(event Custom|FLEE
  (bind _returnvalue (Math|Random|RandomFloatinRange 5e+05 1e+06))
  (bind _defaultsceneroot (Variables|Default|GetDefaultSceneRoot))
  (bind _skeletalmesh (Variables|Default|GetSkeletalMesh))
  (bind _skeletalmesh_2 (Variables|Default|GetSkeletalMesh))
  (bind _defaultsceneroot_2 (Variables|Default|GetDefaultSceneRoot))
  (bind _returnvalue_2 (Transformation|GetWorldLocation _defaultsceneroot))
  (bind _returnvalue_3 (+ _returnvalue_2 "0.000000,0.000000,100.000000"))
  ;[0 0.2291 1] FLEE
  (Utilities|FlowControl|Sequence
    (:then_0
      (goto _label Stop))
    (:then_1
      (if (not (Variables|Default|GetBaloonINVIN))
        (Variables|Default|SetBaloonINVIN true)
        (Variables|Default|SetBaloonKILL false)
        ;;[0 0 0 0.5] Sound
        (Audio|PlaySoundatLocation (.OutItem (Utilities|Array|Random (Utilities|Array|MakeArray "/Game/NotewatchContent/Audio/Sounds/Baloon1.Baloon1" "/Game/NotewatchContent/Audio/Sounds/Baloon2.Baloon2" "/Game/NotewatchContent/Audio/Sounds/Baloon3.Baloon3"))) _returnvalue_2 "0, 0, 0" (Math|Random|RandomFloatinRange 0.5 1.0) (Math|Random|RandomFloatinRange 0.5 1.5) 0.0 0 0 0 0)
        (Components|Animation|PlayAnimation _skeletalmesh "/Game/NotewatchContent/Monsters/Baloon/Other/Baloon_Anim.Baloon_Anim" true)
        (Components|Timeline|SetPlayRate _skeletalmesh 0.5)
        (Components|MoveComponentTo (Variables|Default|GetDefaultSceneRoot) "0.000000,0.000000,35000.000000" (Math|Rotator|MakeRotator 9e+01 0.0 0.0) false true 5.0 false)
        (switch int (Math|Random|RandomIntegerinRange 0 1)
          (:0
            (Components|MoveComponentTo (Variables|Default|GetDefaultSceneRoot) _returnvalue_3 (Math|Rotator|MakeRotator 0.0 0.0 1.3e+02) false true 5.0 false)
            (Components|MoveComponentTo _defaultsceneroot (+ _returnvalue_2 (Math|Vector|MakeVector 2.5e+06 2.5e+06 _returnvalue)) (Math|Rotator|MakeRotator 0.0 (Math|Random|RandomFloatinRange -3.6e+03 3.6e+02) 1.3e+02) false true 15.0 false))
          (:1
            (Components|MoveComponentTo (Variables|Default|GetDefaultSceneRoot) _returnvalue_3 (Math|Rotator|MakeRotator 0.0 0.0 -4e+01) false true 5.0 false)
            (Components|MoveComponentTo (Variables|Default|GetDefaultSceneRoot) (+ "" (Math|Vector|MakeVector -2.5e+06 -2.5e+06 _returnvalue)) (Math|Rotator|MakeRotator 0.0 0.0 -4e+01) false true 15.0 false)))
        (Variables|Default|SetStartLOC "0.000000,0.000000,-50000.000000")
        (Transformation|SetWorldLocation _defaultsceneroot (Variables|Default|GetStartLOC) false true)
        (Transformation|SetActorLocation (Variables|Default|GetStartLOC) false true)
        (Utilities|FlowControl|Delay (Math|Random|RandomFloatinRange 4e+01 8e+01))
        (Variables|Default|SetBaloonINVIN false)
        (Variables|Default|SetBaloonKILL false)
        ;[1 0.2527 0.8639] HUNT
        ;;[0 0 0 0.5] Sound
        (Audio|PlaySoundatLocation (.OutItem (Utilities|Array|Random (Utilities|Array|MakeArray "/Game/NotewatchContent/Audio/Sounds/Baloon1.Baloon1" "/Game/NotewatchContent/Audio/Sounds/Baloon2.Baloon2" "/Game/NotewatchContent/Audio/Sounds/Baloon3.Baloon3"))) _returnvalue_2 "0, 0, 0" (Math|Random|RandomFloatinRange 0.25 0.25) (Math|Random|RandomFloatinRange 0.5 1.0) 0.0 0 0 0 0)
        (Components|Animation|PlayAnimation _skeletalmesh_2 "/Game/NotewatchContent/Monsters/Baloon/Other/Baloon_Anim.Baloon_Anim" true)
        (Components|Timeline|SetPlayRate _skeletalmesh_2 0.25)
        (switch int (Math|Random|RandomIntegerinRange 0 2)
          (:0
            (Variables|Default|SetStartLOC (Variables|Default|GetLOC1))
            (Variables|Default|SetStartROT (Variables|Default|GetROT1)))
          (:1
            (Variables|Default|SetStartLOC (Variables|Default|GetLOC2))
            (Variables|Default|SetStartROT (Variables|Default|GetROT2)))
          (:2
            (Variables|Default|SetStartLOC (Variables|Default|GetLOC3))
            (Variables|Default|SetStartROT (Variables|Default|GetROT3))))
        (Transformation|SetActorLocationAndRotation (+ (Variables|Default|GetStartLOC) "0.000000,0.000000,100000.000000") "0.000000,0.000000,180.000000" false true)
        (Transformation|SetWorldLocation _defaultsceneroot_2 (+ (Variables|Default|GetStartLOC) "0.000000,0.000000,100000.000000") false true)
        (Components|MoveComponentTo _defaultsceneroot_2 (Variables|Default|GetStartLOC) (Variables|Default|GetStartROT) true true 15.0 false :!label _label)
        (Variables|Default|SetBaloonKILL true)
        (Utilities|FlowControl|RetriggerableDelay (Math|Random|RandomFloatinRange 3e+01 3e+01))
        (if (not (Variables|Default|GetBaloonINVIN))
          (if (Variables|Default|GetBaloonKILL)
            (CallFunction|DIE)))))))

(event Custom|HUNT
  (bind _skeletalmesh (Variables|Default|GetSkeletalMesh))
  (bind _defaultsceneroot (Variables|Default|GetDefaultSceneRoot))
  ;[1 0.2527 0.8639] HUNT
  (Utilities|FlowControl|Delay (Math|Random|RandomFloatinRange 1e+02 2e+02))
  ;;[0 0 0 0.5] Sound
  (Audio|PlaySoundatLocation (.OutItem (Utilities|Array|Random (Utilities|Array|MakeArray "/Game/NotewatchContent/Audio/Sounds/Baloon1.Baloon1" "/Game/NotewatchContent/Audio/Sounds/Baloon2.Baloon2" "/Game/NotewatchContent/Audio/Sounds/Baloon3.Baloon3"))) (Transformation|GetWorldLocation (Variables|Default|GetDefaultSceneRoot)) "0, 0, 0" (Math|Random|RandomFloatinRange 0.25 0.25) (Math|Random|RandomFloatinRange 0.5 1.0) 0.0 0 0 0 0)
  (Components|Animation|PlayAnimation _skeletalmesh "/Game/NotewatchContent/Monsters/Baloon/Other/Baloon_Anim.Baloon_Anim" true)
  (Components|Timeline|SetPlayRate _skeletalmesh 0.25)
  (switch int (Math|Random|RandomIntegerinRange 0 2)
    (:0
      (Variables|Default|SetStartLOC (Variables|Default|GetLOC1))
      (Variables|Default|SetStartROT (Variables|Default|GetROT1)))
    (:1
      (Variables|Default|SetStartLOC (Variables|Default|GetLOC2))
      (Variables|Default|SetStartROT (Variables|Default|GetROT2)))
    (:2
      (Variables|Default|SetStartLOC (Variables|Default|GetLOC3))
      (Variables|Default|SetStartROT (Variables|Default|GetROT3))))
  (Transformation|SetActorLocationAndRotation (+ (Variables|Default|GetStartLOC) "0.000000,0.000000,100000.000000") "0.000000,0.000000,180.000000" false true)
  (Transformation|SetWorldLocation _defaultsceneroot (+ (Variables|Default|GetStartLOC) "0.000000,0.000000,100000.000000") false true)
  (Components|MoveComponentTo _defaultsceneroot (Variables|Default|GetStartLOC) (Variables|Default|GetStartROT) true true 15.0 false)
  (Variables|Default|SetBaloonKILL true)
  (Utilities|FlowControl|RetriggerableDelay (Math|Random|RandomFloatinRange 3e+01 3e+01))
  (if (not (Variables|Default|GetBaloonINVIN))
    (if (Variables|Default|GetBaloonKILL)
      (CallFunction|DIE))))

(event Custom|DIE
  (bind _returnvalue (Math|Random|RandomFloatinRange 1.5 1.5))
  (bind _returnvalue_2 (Math|Random|RandomFloatinRange 2.0 2.0))
  (bind _skeletalmesh (Variables|Default|GetSkeletalMesh))
  (bind _defaultsceneroot (Variables|Default|GetDefaultSceneRoot))
  (bind _returnvalue_3 (Transformation|GetWorldLocation _defaultsceneroot))
  ;[1 0 0.005053] Comment
  (Variables|Default|SetBaloonINVIN true)
  ;;[0 0 0 0.5] Sound
  (Audio|PlaySoundatLocation (.OutItem (Utilities|Array|Random (Utilities|Array|MakeArray "/Game/NotewatchContent/Audio/Sounds/Baloon1.Baloon1" "/Game/NotewatchContent/Audio/Sounds/Baloon2.Baloon2" "/Game/NotewatchContent/Audio/Sounds/Baloon3.Baloon3"))) _returnvalue_3 "0, 0, 0" (Math|Random|RandomFloatinRange 1.5 1.5) (Math|Random|RandomFloatinRange 1.75 2.0) 0.0 0 0 0 0)
  (Components|Animation|PlayAnimation _skeletalmesh "/Game/NotewatchContent/Monsters/Baloon/Other/Baloon_Anim.Baloon_Anim" true)
  (Components|Timeline|SetPlayRate _skeletalmesh 0.5)
  (Components|MoveComponentTo (Variables|Default|GetDefaultSceneRoot) "0.000000,0.000000,50000.000000" (Math|Rotator|MakeRotator 9e+01 0.0 0.0) false true 5.0 false)
  (Components|MoveComponentTo (Variables|Default|GetDefaultSceneRoot) "0.000000,0.000000,50000.000000" (Math|Rotator|MakeRotator -9e+01 2.4e+02 0.0) false true 1.0 false)
  (Utilities|FlowControl|Delay (Math|Random|RandomFloatinRange 1.0 25.0))
  (bind _returnvalue_4 (Actor|GetActorOfClass "/Game/FirstPerson/Blueprints/BP_FirstPersonCharacter.BP_FirstPersonCharacter_C"))
  (Pawn|SetControlRotation (Game|GetPlayerController (Variables|/Script/Engine.Pawn|GetPlayerState _returnvalue_4)) (Math|Rotator|FindLookatRotation (Transformation|GetWorldLocation (Variables|/Game/FirstPerson/Blueprints/BP_FirstPersonCharacter.BP_FirstPersonCharacter_C|GetFirstPersonCamera _returnvalue_4)) _returnvalue_3))
  (Pawn|Components|CharacterMovement|DisableMovement (Variables|/Script/Engine.Character|GetCharacterMovement _returnvalue_4))
  ;;[0 0 0 0.5] Sound
  (Audio|PlaySoundatLocation "/Game/NotewatchContent/Audio/Sounds/Baloon2.Baloon2" "0, 0, 0" "0.000000,0.000000,-90.000000" _returnvalue _returnvalue_2 1.5 0 0 0 0)
  (Audio|PlaySoundatLocation "/Game/NotewatchContent/Audio/Sounds/Baloon2.Baloon2" _returnvalue_3 "0.000000,0.000000,-90.000000" _returnvalue _returnvalue_2 1.5 0 0 0 0)
  (Audio|PlaySoundatLocation "/Game/NotewatchContent/Audio/Sounds/Baloon1.Baloon1" _returnvalue_3 "0.000000,0.000000,-90.000000" _returnvalue _returnvalue_2 1.5 0 0 0 0)
  (Components|MoveComponentTo (Variables|Default|GetDefaultSceneRoot) (Variables|Default|GetKillLOC) (Variables|Default|GetKillROT) true false 1.0 true)
  (Default|DIE _returnvalue_4))

(fn ConstructionScript)