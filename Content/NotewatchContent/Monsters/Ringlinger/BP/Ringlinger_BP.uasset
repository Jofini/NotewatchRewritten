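; Ringlinger monster Blueprint that slowly descends from high in the sky onto one of three preset spots and threatens the player.
; HUNT starts the descent after a random delay; arrival arms a timed kill.
; FLEE halts it, flies the monster away, hides it, then restarts the cycle, with flags guarding re-entry.
; DIE turns the player's view toward it, freezes movement, lunges at the camera and kills the player.
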(event Custom|FLEE
  (bind _returnvalue (Math|Random|RandomFloatinRange -15.0 15.0))
  (bind _returnvalue_2 (Math|Random|RandomFloatinRange -2.5e+03 2.5e+03))
  (bind _skeletalmesh (Variables|Default|GetSkeletalMesh))
  (bind _defaultsceneroot (Variables|Default|GetDefaultSceneRoot))
  (bind _skeletalmesh_2 (Variables|Default|GetSkeletalMesh))
  (bind _defaultsceneroot_2 (Variables|Default|GetDefaultSceneRoot))
  (bind _returnvalue_3 (Transformation|GetWorldLocation _defaultsceneroot))
  ;[0 0.2291 1] FLEE
  (Utilities|FlowControl|Sequence
    (:then_0
      (goto _label Stop))
    (:then_1
      (if (not (Variables|Default|GetRLingINVIN))
        (Variables|Default|SetRLingINVIN true)
        (Variables|Default|SetRLingKILL false)
        ;;[0 0 0 0.5] Sound
        (Audio|PlaySoundatLocation (.OutItem (Utilities|Array|Random (Utilities|Array|MakeArray "/Game/NotewatchContent/Audio/Sounds/Ringlinger1.Ringlinger1" "/Game/NotewatchContent/Audio/Sounds/Ringlinger2.Ringlinger2" "/Game/NotewatchContent/Audio/Sounds/Ringlinger3.Ringlinger3"))) _returnvalue_3 "0, 0, 0" (Math|Random|RandomFloatinRange 0.25 1.0) (Math|Random|RandomFloatinRange 0.25 2.0) 0.0 0 0 0 0)
        (Components|Timeline|SetPlayRate _skeletalmesh 0.5)
        (Components|Animation|PlayAnimation _skeletalmesh "/Game/NotewatchContent/Monsters/Ringlinger/Other/Run.Run" true)
        (Components|MoveComponentTo _defaultsceneroot (+ _returnvalue_3 (Math|Vector|MakeVector _returnvalue_2 _returnvalue_2 2e+03)) (Math|Rotator|MakeRotator 9e+01 _returnvalue _returnvalue) true true 2.5 true)
        (Components|MoveComponentTo _defaultsceneroot (+ _returnvalue_3 (Math|Vector|MakeVector _returnvalue_2 _returnvalue_2 1e+05)) (Math|Rotator|MakeRotator 3.6e+02 _returnvalue _returnvalue) true true 25.0 true)
        (Variables|Default|SetStartLOC "0.000000,0.000000,-50000.000000")
        (Transformation|SetWorldLocation _defaultsceneroot (Variables|Default|GetStartLOC) false true)
        (Transformation|SetActorLocation (Variables|Default|GetStartLOC) false true)
        (Utilities|FlowControl|Delay (Math|Random|RandomFloatinRange 2e+01 4e+01))
        (Variables|Default|SetRLingINVIN false)
        (Variables|Default|SetRLingKILL false)
        ;[1 0.2527 0.8639] HUNT
        (Components|Animation|PlayAnimation _skeletalmesh_2 "/Game/NotewatchContent/Monsters/Ringlinger/Other/Idle.Idle" true)
        (Components|Timeline|SetPlayRate _skeletalmesh_2 0.25)
        (switch int (Math|Random|RandomIntegerinRange 0 2)
          (:0
            (Variables|Default|SetStartLOC (Variables|Default|GetLOC1))
            (Variables|Default|SetStartROT (Variables|Default|GetROT1)))
          (:1
            (Variables|Default|SetStartLOC (Variables|Default|GetLOC2))
            (Variables|Default|SetStartROT (Variables|Default|GetROT2)))
          (:2
            (Variables|Default|SetStartLOC (Variables|Default|GetLOC3))
            (Variables|Default|SetStartROT (Variables|Default|GetROT3))))
        (Transformation|SetActorLocationAndRotation (+ (Variables|Default|GetStartLOC) "0.000000,0.000000,100000.000000") (Math|Rotator|MakeRotator (.roll (Variables|Default|GetStartROT)) (.pitch (Variables|Default|GetStartROT)) (.yaw (Variables|Default|GetStartROT))) false true)
        (Transformation|SetWorldLocationAndRotation _defaultsceneroot_2 (+ (Variables|Default|GetStartLOC) "0.000000,0.000000,100000.000000") (Math|Rotator|MakeRotator -1.2e+02 (.pitch (Variables|Default|GetStartROT)) (.yaw (Variables|Default|GetStartROT))) false true)
        (Components|MoveComponentTo _defaultsceneroot_2 (Variables|Default|GetStartLOC) (Variables|Default|GetStartROT) true true 45.0 false :!label _label)
        (Variables|Default|SetRLingKILL true)
        (Utilities|FlowControl|RetriggerableDelay (Math|Random|RandomFloatinRange 3e+01 3e+01))
        (if (not (Variables|Default|GetRLingINVIN))
          (if (Variables|Default|GetRLingKILL)
            (CallFunction|DIE)))))))

(event Custom|HUNT
  (bind _skeletalmesh (Variables|Default|GetSkeletalMesh))
  (bind _defaultsceneroot (Variables|Default|GetDefaultSceneRoot))
  ;[1 0.2527 0.8639] HUNT
  (Utilities|FlowControl|Delay (Math|Random|RandomFloatinRange 4e+01 8e+01))
  (Components|Animation|PlayAnimation _skeletalmesh "/Game/NotewatchContent/Monsters/Ringlinger/Other/Idle.Idle" true)
  (Components|Timeline|SetPlayRate _skeletalmesh 0.25)
  (switch int (Math|Random|RandomIntegerinRange 0 2)
    (:0
      (Variables|Default|SetStartLOC (Variables|Default|GetLOC1))
      (Variables|Default|SetStartROT (Variables|Default|GetROT1)))
    (:1
      (Variables|Default|SetStartLOC (Variables|Default|GetLOC2))
      (Variables|Default|SetStartROT (Variables|Default|GetROT2)))
    (:2
      (Variables|Default|SetStartLOC (Variables|Default|GetLOC3))
      (Variables|Default|SetStartROT (Variables|Default|GetROT3))))
  (Transformation|SetActorLocationAndRotation (+ (Variables|Default|GetStartLOC) "0.000000,0.000000,100000.000000") (Math|Rotator|MakeRotator (.roll (Variables|Default|GetStartROT)) (.pitch (Variables|Default|GetStartROT)) (.yaw (Variables|Default|GetStartROT))) false true)
  (Transformation|SetWorldLocationAndRotation _defaultsceneroot (+ (Variables|Default|GetStartLOC) "0.000000,0.000000,100000.000000") (Math|Rotator|MakeRotator -1.2e+02 (.pitch (Variables|Default|GetStartROT)) (.yaw (Variables|Default|GetStartROT))) false true)
  (Components|MoveComponentTo _defaultsceneroot (Variables|Default|GetStartLOC) (Variables|Default|GetStartROT) true true 45.0 false)
  (Variables|Default|SetRLingKILL true)
  (Utilities|FlowControl|RetriggerableDelay (Math|Random|RandomFloatinRange 3e+01 3e+01))
  (if (not (Variables|Default|GetRLingINVIN))
    (if (Variables|Default|GetRLingKILL)
      (CallFunction|DIE))))

(event Custom|DIE
  ;[1 0 0.005053] Kill
  (Variables|Default|SetRLingINVIN false)
  (bind _returnvalue (Actor|GetActorOfClass "/Game/FirstPerson/Blueprints/BP_FirstPersonCharacter.BP_FirstPersonCharacter_C"))
  (Pawn|SetControlRotation (Game|GetPlayerController (Variables|/Script/Engine.Pawn|GetPlayerState _returnvalue)) (Math|Rotator|FindLookatRotation (Transformation|GetWorldLocation (Variables|/Game/FirstPerson/Blueprints/BP_FirstPersonCharacter.BP_FirstPersonCharacter_C|GetFirstPersonCamera _returnvalue)) (Transformation|GetWorldLocation (Variables|Default|GetDefaultSceneRoot))))
  (Pawn|Components|CharacterMovement|DisableMovement (Variables|/Script/Engine.Character|GetCharacterMovement _returnvalue))
  ;;[0 0 0 0.5] Sound
  (Audio|PlaySoundatLocation (.OutItem (Utilities|Array|Random (Utilities|Array|MakeArray "/Game/NotewatchContent/Audio/Sounds/Ringlinger1.Ringlinger1" "/Game/NotewatchContent/Audio/Sounds/Ringlinger2.Ringlinger2" "/Game/NotewatchContent/Audio/Sounds/Ringlinger3.Ringlinger3"))) (Transformation|GetWorldLocation (Variables|/Game/FirstPerson/Blueprints/BP_FirstPersonCharacter.BP_FirstPersonCharacter_C|GetFirstPersonCamera _returnvalue)) "0, 0, 0" (Math|Random|RandomFloatinRange 1.5 1.5) (Math|Random|RandomFloatinRange 1.25 1.5) 0.0 0 0 0 0)
  (Components|MoveComponentTo (Variables|Default|GetDefaultSceneRoot) (Transformation|GetWorldLocation (Variables|/Game/FirstPerson/Blueprints/BP_FirstPersonCharacter.BP_FirstPersonCharacter_C|GetFirstPersonCamera _returnvalue)) (Variables|Default|GetStartROT) false false 0.5 true)
  (Default|DIE _returnvalue))

(fn ConstructionScript)