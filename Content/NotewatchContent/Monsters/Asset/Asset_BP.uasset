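; Monster that poses as a random primitive mesh and kills the player if it is not made to flee in time.
; HUNT waits, prints an uneasy message, then places it at one of three locations with random shape, scale and rotation.
; FLEE hides it far below the world, prints garbled text and respawns it later.
; A retriggerable timer calls DIE, which turns the player's view toward it, disables movement and kills them.
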(event Custom|FLEE
  (bind _returnvalue (Math|Random|RandomFloatinRange 0.5 5.0))
  ;[0 0.2291 1] FLEE
  (if (not (Variables|Default|GetAFLEEING))
    (Variables|Default|SetAFLEEING true)
    (Variables|Default|SetAKILL false)
    (Utilities|FlowControl|Sequence
      (:then_0
        (switch int (Math|Random|RandomIntegerinRange 0 4)
          (:0
            (Development|PrintString "$21" true true "(R=1.000000,G=1.000000,B=1.000000,A=1.000000)"))
          (:1
            (Development|PrintString "8*%" true true "(R=1.000000,G=1.000000,B=1.000000,A=1.000000)"))
          (:2
            (Development|PrintString "@#!" true true "(R=1.000000,G=1.000000,B=1.000000,A=1.000000)"))
          (:3
            (Development|PrintString "(01" true true "(R=1.000000,G=1.000000,B=1.000000,A=1.000000)"))
          (:4
            (Development|PrintString "\\Q^" true true "(R=1.000000,G=1.000000,B=1.000000,A=1.000000)"))))
      (:then_1
        (Variables|Default|SetStartLOC "0.000000,0.000000,-10000.000000")
        (Transformation|SetWorldLocation (Variables|Default|GetDefaultSceneRoot) (Variables|Default|GetStartLOC) false true)
        (Transformation|SetActorLocation (Variables|Default|GetStartLOC) false true)
        (Utilities|FlowControl|Delay (Math|Random|RandomFloatinRange 3e+01 6e+01))
        (Variables|Default|SetAFLEEING false)
        (Variables|Default|SetAKILL false)
        ;[1 0.2527 0.8639] HUNT
        (switch int (Math|Random|RandomIntegerinRange 0 2)
          (:0
            (Variables|Default|SetStartLOC (Variables|Default|GetLOC1)))
          (:1
            (Variables|Default|SetStartLOC (Variables|Default|GetLOC2)))
          (:2
            (Variables|Default|SetStartLOC (Variables|Default|GetLOC3))))
        (Components|StaticMesh|SetStaticMesh (Variables|Default|GetStaticMesh) (.OutItem (Utilities|Array|Random (Utilities|Array|MakeArray "/Game/StarterContent/Shapes/Shape_Cone.Shape_Cone" "/Game/StarterContent/Architecture/Pillar_50x500.Pillar_50x500" "/Game/StarterContent/Shapes/Shape_Cube.Shape_Cube" "/Game/StarterContent/Shapes/Shape_Cylinder.Shape_Cylinder" "/Game/StarterContent/Shapes/Shape_NarrowCapsule.Shape_NarrowCapsule" "/Game/StarterContent/Shapes/Shape_QuadPyramid.Shape_QuadPyramid" "/Game/StarterContent/Shapes/Shape_Sphere.Shape_Sphere" "/Game/StarterContent/Shapes/Shape_Tube.Shape_Tube" "/Game/StarterContent/Shapes/Shape_Torus.Shape_Torus"))))
        (Transformation|SetActorScale3D (Math|Vector|MakeVector _returnvalue _returnvalue _returnvalue))
        (Transformation|SetWorldLocationAndRotation (Variables|Default|GetDefaultSceneRoot) (Variables|Default|GetStartLOC) (Math|Random|RandomRotator true) false true)
        (Variables|Default|SetAKILL true)
        (Utilities|FlowControl|RetriggerableDelay (Math|Random|RandomFloatinRange 3e+01 3e+01))
        (if (Variables|Default|GetAKILL)
          (CallFunction|DIE))))))

(event Custom|HUNT
  (bind _returnvalue (Math|Random|RandomFloatinRange 0.5 5.0))
  ;[1 0.2527 0.8639] HUNT
  (if (not (Variables|Default|GetAFLEEING))
    (Utilities|FlowControl|Delay (Math|Random|RandomFloatinRange 6e+01 1.2e+02))
    (Utilities|FlowControl|Sequence
      (:then_0
        (switch int (Math|Random|RandomIntegerinRange 0 4)
          (:0
            (Development|PrintString "Hello?" true true "(R=1.000000,G=1.000000,B=1.000000,A=1.000000)"))
          (:1
            (Development|PrintString "Why?" true true "(R=1.000000,G=1.000000,B=1.000000,A=1.000000)"))
          (:2
            (Development|PrintString "Are you okay?" true true "(R=1.000000,G=1.000000,B=1.000000,A=1.000000)"))
          (:3
            (Development|PrintString "Do you see me?" true true "(R=1.000000,G=1.000000,B=1.000000,A=1.000000)"))
          (:4
            (Development|PrintString "Where am I?" true true "(R=1.000000,G=1.000000,B=1.000000,A=1.000000)"))))
      (:then_1
        (switch int (Math|Random|RandomIntegerinRange 0 2)
          (:0
            (Variables|Default|SetStartLOC (Variables|Default|GetLOC1)))
          (:1
            (Variables|Default|SetStartLOC (Variables|Default|GetLOC2)))
          (:2
            (Variables|Default|SetStartLOC (Variables|Default|GetLOC3))))
        (Components|StaticMesh|SetStaticMesh (Variables|Default|GetStaticMesh) (.OutItem (Utilities|Array|Random (Utilities|Array|MakeArray "/Game/StarterContent/Shapes/Shape_Cone.Shape_Cone" "/Game/StarterContent/Architecture/Pillar_50x500.Pillar_50x500" "/Game/StarterContent/Shapes/Shape_Cube.Shape_Cube" "/Game/StarterContent/Shapes/Shape_Cylinder.Shape_Cylinder" "/Game/StarterContent/Shapes/Shape_NarrowCapsule.Shape_NarrowCapsule" "/Game/StarterContent/Shapes/Shape_QuadPyramid.Shape_QuadPyramid" "/Game/StarterContent/Shapes/Shape_Sphere.Shape_Sphere" "/Game/StarterContent/Shapes/Shape_Tube.Shape_Tube" "/Game/StarterContent/Shapes/Shape_Torus.Shape_Torus"))))
        (Transformation|SetActorScale3D (Math|Vector|MakeVector _returnvalue _returnvalue _returnvalue))
        (Transformation|SetWorldLocationAndRotation (Variables|Default|GetDefaultSceneRoot) (Variables|Default|GetStartLOC) (Math|Random|RandomRotator true) false true)
        (Variables|Default|SetAKILL true)
        (Utilities|FlowControl|RetriggerableDelay (Math|Random|RandomFloatinRange 3e+01 3e+01))
        (if (Variables|Default|GetAKILL)
          (CallFunction|DIE))))))

(event Custom|DIE
  ;[1 0 0.005053] Comment
  (bind _returnvalue (Actor|GetActorOfClass "/Game/FirstPerson/Blueprints/BP_FirstPersonCharacter.BP_FirstPersonCharacter_C"))
  (Pawn|SetControlRotation (Game|GetPlayerController (Variables|/Script/Engine.Pawn|GetPlayerState _returnvalue)) (Math|Rotator|FindLookatRotation (Transformation|GetWorldLocation (Variables|/Game/FirstPerson/Blueprints/BP_FirstPersonCharacter.BP_FirstPersonCharacter_C|GetFirstPersonCamera _returnvalue)) (Transformation|GetWorldLocation (Variables|Default|GetDefaultSceneRoot))))
  (Pawn|Components|CharacterMovement|DisableMovement (Variables|/Script/Engine.Character|GetCharacterMovement _returnvalue))
  (Default|DIE _returnvalue))

(fn ConstructionScript)