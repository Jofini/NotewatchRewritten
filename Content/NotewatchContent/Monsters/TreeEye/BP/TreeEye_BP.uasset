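; TreeEye monster that periodically appears at one of three preset spots and punishes the player if not driven off in time.
; FLEE plays a pitch-varied sound, hides the actor far below the world, then respawns it after random delays; HUNT enters at the respawn wait.
; If still armed when its timer expires, DIE locks the player's view onto it through Tick, blocking FLEE, then releases and flees.
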(event Custom|FLEE
  (bind _returnvalue (Math|Random|RandomFloatinRange 0.25 0.5))
  (bind _defaultsceneroot (Variables|Default|GetDefaultSceneRoot))
  (bind _returnvalue_2 (Transformation|GetWorldLocation _defaultsceneroot))
  ;[0 0.2291 1] FLEE
  (if (not (Variables|Default|GetLookAtTreeEye))
    (if (not (Variables|Default|GetTEFLEEING))
      (Variables|Default|SetTEFLEEING true)
      (Variables|Default|SetTEKILL false)
      ;;[0 0 0 0.5] Sound
      (Audio|PlaySoundatLocation "/Game/NotewatchContent/Audio/Sounds/TreeEye.TreeEye" _returnvalue_2 "0, 0, 0" (Math|Random|RandomFloatinRange 0.5 1.0) (Math|Random|RandomFloatinRange 0.5 1.5) 0.0 0 0 0 0)
      (Variables|Default|SetStartLOC "0.000000,0.000000,-50000.000000")
      (Transformation|SetWorldLocation _defaultsceneroot (Variables|Default|GetStartLOC) false true)
      (Transformation|SetActorLocation (Variables|Default|GetStartLOC) false true)
      (Utilities|FlowControl|Delay (Math|Random|RandomFloatinRange 1e+01 2e+01))
      (Variables|Default|SetTEFLEEING false)
      (Variables|Default|SetTEKILL false)
      ;[1 0.2527 0.8639] HUNT
      (Utilities|FlowControl|Delay (Math|Random|RandomFloatinRange 45.0 9e+01))
      (switch int (Math|Random|RandomIntegerinRange 0 2)
        (:0
          (Variables|Default|SetStartLOC (Variables|Default|GetLOC1))
          (Variables|Default|SetStartROT (Variables|Default|GetROT1)))
        (:1
          (Variables|Default|SetStartLOC (Variables|Default|GetLOC2))
          (Variables|Default|SetStartROT (Variables|Default|GetROT2)))
        (:2
          (Variables|Default|SetStartLOC (Variables|Default|GetLOC3))
          (Variables|Default|SetStartROT (Variables|Default|GetROT3))))
      (Transformation|SetActorLocationAndRotation (Variables|Default|GetStartLOC) (Variables|Default|GetStartROT) false true)
      (Transformation|SetWorldLocation (Variables|Default|GetDefaultSceneRoot) (Variables|Default|GetStartLOC) false true)
      ;;[0 0 0 0.5] Sound
      (Audio|PlaySoundatLocation "/Game/NotewatchContent/Audio/Sounds/TreeEye.TreeEye" _returnvalue_2 "0, 0, 0" _returnvalue _returnvalue 0.0 0 0 0 0)
      (Variables|Default|SetTEKILL true)
      (Utilities|FlowControl|RetriggerableDelay (Math|Random|RandomFloatinRange 15.0 15.0))
      (if (Variables|Default|GetTEKILL)
        (CallFunction|DIE)))))

(event Custom|HUNT
  (bind _returnvalue (Math|Random|RandomFloatinRange 0.25 0.5))
  ;[1 0.2527 0.8639] HUNT
  (if (not (Variables|Default|GetTEFLEEING))
    (Utilities|FlowControl|Delay (Math|Random|RandomFloatinRange 45.0 9e+01))
    (switch int (Math|Random|RandomIntegerinRange 0 2)
      (:0
        (Variables|Default|SetStartLOC (Variables|Default|GetLOC1))
        (Variables|Default|SetStartROT (Variables|Default|GetROT1)))
      (:1
        (Variables|Default|SetStartLOC (Variables|Default|GetLOC2))
        (Variables|Default|SetStartROT (Variables|Default|GetROT2)))
      (:2
        (Variables|Default|SetStartLOC (Variables|Default|GetLOC3))
        (Variables|Default|SetStartROT (Variables|Default|GetROT3))))
    (Transformation|SetActorLocationAndRotation (Variables|Default|GetStartLOC) (Variables|Default|GetStartROT) false true)
    (Transformation|SetWorldLocation (Variables|Default|GetDefaultSceneRoot) (Variables|Default|GetStartLOC) false true)
    ;;[0 0 0 0.5] Sound
    (Audio|PlaySoundatLocation "/Game/NotewatchContent/Audio/Sounds/TreeEye.TreeEye" (Transformation|GetWorldLocation (Variables|Default|GetDefaultSceneRoot)) "0, 0, 0" _returnvalue _returnvalue 0.0 0 0 0 0)
    (Variables|Default|SetTEKILL true)
    (Utilities|FlowControl|RetriggerableDelay (Math|Random|RandomFloatinRange 15.0 15.0))
    (if (Variables|Default|GetTEKILL)
      (CallFunction|DIE))))

(event Custom|DIE
  (bind _returnvalue (Math|Random|RandomFloatinRange 1.5 1.5))
  (bind _returnvalue_2 (Math|Random|RandomFloatinRange 0.5 1.5))
  (bind _returnvalue_3 (Math|Random|RandomFloatinRange 0.25 0.5))
  (bind _defaultsceneroot (Variables|Default|GetDefaultSceneRoot))
  (bind _returnvalue_4 (Transformation|GetWorldLocation _defaultsceneroot))
  ;[1 0 0.005053] Comment
  (bind _returnvalue_5 (Actor|GetActorOfClass "/Game/FirstPerson/Blueprints/BP_FirstPersonCharacter.BP_FirstPersonCharacter_C"))
  ;;[0 0 0] Sound
  (Audio|PlaySoundatLocation "/Game/NotewatchContent/Audio/Sounds/TreeEye.TreeEye" _returnvalue_4 "0, 0, 0" _returnvalue _returnvalue_2 0.0 0 0 0 0)
  (Pawn|SetControlRotation (Game|GetPlayerController (Variables|/Script/Engine.Pawn|GetPlayerState _returnvalue_5)) (Math|Rotator|FindLookatRotation (Transformation|GetWorldLocation (Variables|/Game/FirstPerson/Blueprints/BP_FirstPersonCharacter.BP_FirstPersonCharacter_C|GetFirstPersonCamera _returnvalue_5)) (Transformation|GetWorldLocation (Variables|Default|GetDefaultSceneRoot))))
  (Variables|Default|SetLookAtTreeEye true)
  (Utilities|FlowControl|Delay 5.0)
  (Variables|Default|SetLookAtTreeEye false)
  (Audio|PlaySoundatLocation "/Game/NotewatchContent/Audio/Sounds/TreeEye.TreeEye" _returnvalue_4 "0, 0, 0" _returnvalue _returnvalue_2 0.0 0 0 0 0)
  ;[0 0.2291 1] FLEE
  (if (not (Variables|Default|GetTEFLEEING))
    (Variables|Default|SetTEFLEEING true)
    (Variables|Default|SetTEKILL false)
    ;;[0 0 0 0.5] Sound
    (Audio|PlaySoundatLocation "/Game/NotewatchContent/Audio/Sounds/TreeEye.TreeEye" _returnvalue_4 "0, 0, 0" (Math|Random|RandomFloatinRange 0.5 1.0) (Math|Random|RandomFloatinRange 0.5 1.5) 0.0 0 0 0 0)
    (Variables|Default|SetStartLOC "0.000000,0.000000,-50000.000000")
    (Transformation|SetWorldLocation _defaultsceneroot (Variables|Default|GetStartLOC) false true)
    (Transformation|SetActorLocation (Variables|Default|GetStartLOC) false true)
    (Utilities|FlowControl|Delay (Math|Random|RandomFloatinRange 1e+01 2e+01))
    (Variables|Default|SetTEFLEEING false)
    (Variables|Default|SetTEKILL false)
    ;[1 0.2527 0.8639] HUNT
    (Utilities|FlowControl|Delay (Math|Random|RandomFloatinRange 45.0 9e+01))
    (switch int (Math|Random|RandomIntegerinRange 0 2)
      (:0
        (Variables|Default|SetStartLOC (Variables|Default|GetLOC1))
        (Variables|Default|SetStartROT (Variables|Default|GetROT1)))
      (:1
        (Variables|Default|SetStartLOC (Variables|Default|GetLOC2))
        (Variables|Default|SetStartROT (Variables|Default|GetROT2)))
      (:2
        (Variables|Default|SetStartLOC (Variables|Default|GetLOC3))
        (Variables|Default|SetStartROT (Variables|Default|GetROT3))))
    (Transformation|SetActorLocationAndRotation (Variables|Default|GetStartLOC) (Variables|Default|GetStartROT) false true)
    (Transformation|SetWorldLocation (Variables|Default|GetDefaultSceneRoot) (Variables|Default|GetStartLOC) false true)
    ;;[0 0 0 0.5] Sound
    (Audio|PlaySoundatLocation "/Game/NotewatchContent/Audio/Sounds/TreeEye.TreeEye" _returnvalue_4 "0, 0, 0" _returnvalue_3 _returnvalue_3 0.0 0 0 0 0)
    (Variables|Default|SetTEKILL true)
    (Utilities|FlowControl|RetriggerableDelay (Math|Random|RandomFloatinRange 15.0 15.0))
    (if (Variables|Default|GetTEKILL)
      (CallFunction|DIE))))

(event EventTick
  (params (DeltaSeconds :type Float%20%28single-precision%29))
  (if (Variables|Default|GetLookAtTreeEye)
    (Pawn|SetControlRotation (Game|GetPlayerController (Variables|/Script/Engine.Pawn|GetPlayerState (stale Custom|DIE _returnvalue_5))) (Math|Rotator|FindLookatRotation (Transformation|GetWorldLocation (Variables|/Game/FirstPerson/Blueprints/BP_FirstPersonCharacter.BP_FirstPersonCharacter_C|GetFirstPersonCamera (stale Custom|DIE _returnvalue_5))) (Transformation|GetWorldLocation (Variables|Default|GetDefaultSceneRoot))))))

(fn ConstructionScript)