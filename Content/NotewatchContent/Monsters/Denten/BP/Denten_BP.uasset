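; Denten monster that descends from high above onto one of three spots, then kills the player if not driven off within 30 seconds.
; FLEE makes it invulnerable, sends it skyward and hides it below the map before another descent; HUNT starts a descent after a long random delay.
; DIE yells, freezes the player and lunges, while Tick locks the camera onto the monster.
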(event Custom|FLEE
  (bind _returnvalue (Math|Random|RandomRotator false))
  (bind _returnvalue_2 (Math|Random|RandomRotator false))
  (bind _defaultsceneroot (Variables|Default|GetDefaultSceneRoot))
  (bind _defaultsceneroot_2 (Variables|Default|GetDefaultSceneRoot))
  ;[0 0.2291 1] FLEE
  (Utilities|FlowControl|Sequence
    (:then_0
      (goto _label Stop))
    (:then_1
      (if (not (Variables|Default|GetDentINVIN))
        (Variables|Default|SetDentINVIN true)
        (Variables|Default|SetDentKILL false)
        (Components|Timeline|SetPlayRate (Variables|Default|GetSkeletalMesh) 5.0)
        (Components|MoveComponentTo (Variables|Default|GetDefaultSceneRoot) (Variables|Default|GetStartLOC) _returnvalue_2 true true 1.0 true)
        (Components|MoveComponentTo _defaultsceneroot (+ (Variables|Default|GetStartLOC) "0.000000,0.000000,100000.000000") _returnvalue_2 true true 15.0 true)
        (Variables|Default|SetStartLOC "0.000000,0.000000,-50000.000000")
        (Transformation|SetWorldLocation _defaultsceneroot (Variables|Default|GetStartLOC) false true)
        (Transformation|SetActorLocation (Variables|Default|GetStartLOC) false true)
        (Utilities|FlowControl|Delay (Math|Random|RandomFloatinRange 2e+01 4e+01))
        (Variables|Default|SetDentINVIN false)
        (Variables|Default|SetDentKILL false)
        ;[1 0.2527 0.8639] HUNT
        (Components|Timeline|SetPlayRate (Variables|Default|GetSkeletalMesh) 1.0)
        (switch int (Math|Random|RandomIntegerinRange 0 2)
          (:0
            (Variables|Default|SetStartLOC (Variables|Default|GetLOC1))
            (Variables|Default|SetStartROT (Variables|Default|GetROT1)))
          (:1
            (Variables|Default|SetStartLOC (Variables|Default|GetLOC2))
            (Variables|Default|SetStartROT (Variables|Default|GetROT2)))
          (:2
            (Variables|Default|SetStartLOC (Variables|Default|GetLOC3))
            (Variables|Default|SetStartROT (Variables|Default|GetROT3))))
        (Transformation|SetActorLocationAndRotation (+ (Variables|Default|GetStartLOC) "0.000000,0.000000,100000.000000") _returnvalue false true)
        (Transformation|SetWorldLocation _defaultsceneroot_2 (+ (Variables|Default|GetStartLOC) "0.000000,0.000000,100000.000000") false true)
        (Components|MoveComponentTo _defaultsceneroot_2 (Variables|Default|GetStartLOC) _returnvalue true true 25.0 true :!label _label)
        (Components|MoveComponentTo _defaultsceneroot_2 (Variables|Default|GetStartLOC) _returnvalue true true 1.0 true)
        (Variables|Default|SetDentKILL true)
        (Utilities|FlowControl|RetriggerableDelay (Math|Random|RandomFloatinRange 3e+01 3e+01))
        (if (not (Variables|Default|GetDentINVIN))
          (if (Variables|Default|GetDentKILL)
            (CallFunction|DIE)))))))

(event Custom|HUNT
  (bind _returnvalue (Math|Random|RandomRotator false))
  (bind _defaultsceneroot (Variables|Default|GetDefaultSceneRoot))
  ;[1 0.2527 0.8639] HUNT
  (Utilities|FlowControl|Delay (Math|Random|RandomFloatinRange 3.5e+02 7e+02))
  (Components|Timeline|SetPlayRate (Variables|Default|GetSkeletalMesh) 1.0)
  (switch int (Math|Random|RandomIntegerinRange 0 2)
    (:0
      (Variables|Default|SetStartLOC (Variables|Default|GetLOC1))
      (Variables|Default|SetStartROT (Variables|Default|GetROT1)))
    (:1
      (Variables|Default|SetStartLOC (Variables|Default|GetLOC2))
      (Variables|Default|SetStartROT (Variables|Default|GetROT2)))
    (:2
      (Variables|Default|SetStartLOC (Variables|Default|GetLOC3))
      (Variables|Default|SetStartROT (Variables|Default|GetROT3))))
  (Transformation|SetActorLocationAndRotation (+ (Variables|Default|GetStartLOC) "0.000000,0.000000,100000.000000") _returnvalue false true)
  (Transformation|SetWorldLocation _defaultsceneroot (+ (Variables|Default|GetStartLOC) "0.000000,0.000000,100000.000000") false true)
  (Components|MoveComponentTo _defaultsceneroot (Variables|Default|GetStartLOC) _returnvalue true true 25.0 true)
  (Components|MoveComponentTo _defaultsceneroot (Variables|Default|GetStartLOC) _returnvalue true true 1.0 true)
  (Variables|Default|SetDentKILL true)
  (Utilities|FlowControl|RetriggerableDelay (Math|Random|RandomFloatinRange 3e+01 3e+01))
  (if (not (Variables|Default|GetDentINVIN))
    (if (Variables|Default|GetDentKILL)
      (CallFunction|DIE))))

(event Custom|DIE
  ;[1 0 0.005053] Comment
  (Variables|Default|SetDentINVIN true)
  (Audio|PlaySoundatLocation "/Game/NotewatchContent/Audio/Sounds/DentenYell.DentenYell" (Transformation|GetWorldLocation (Variables|Default|GetDefaultSceneRoot)) "0, 0, 0" 1.0 (Math|Random|RandomFloatinRange 1.5 2.0) 0.0 0 0 0 0)
  (Variables|Default|SetLADent true)
  (Pawn|Components|CharacterMovement|DisableMovement (Variables|/Script/Engine.Character|GetCharacterMovement (stale EventTick _returnvalue)))
  (Components|Timeline|SetPlayRate (Variables|Default|GetSkeletalMesh) 1e+01)
  (Components|MoveComponentTo (Variables|Default|GetDefaultSceneRoot) (- (Transformation|GetActorLocation (stale EventTick _returnvalue)) "0.000000,0.000000,100.000000") (Math|Random|RandomRotator false) false true 1.0 true)
  (Default|DIE (stale EventTick _returnvalue)))

(event EventTick
  (params (DeltaSeconds :type Float%20%28single-precision%29))
  ;[1 0 0.005053] Comment
  (if (Variables|Default|GetLADent)
    (bind _returnvalue (Actor|GetActorOfClass "/Game/FirstPerson/Blueprints/BP_FirstPersonCharacter.BP_FirstPersonCharacter_C"))
    (Pawn|SetControlRotation (Game|GetPlayerController (Variables|/Script/Engine.Pawn|GetPlayerState _returnvalue)) (Math|Rotator|FindLookatRotation (Transformation|GetWorldLocation (Variables|/Game/FirstPerson/Blueprints/BP_FirstPersonCharacter.BP_FirstPersonCharacter_C|GetFirstPersonCamera _returnvalue)) (Transformation|GetWorldLocation (Variables|Default|GetDefaultSceneRoot))))))

(fn ConstructionScript)