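; Roboach monster actor that drops in at one of three preset spots and kills the player if not scared off in time.
; FLEE starts the game on first call, then lifts Roboach away with sound and Niagara, hides it far below and re-enters the hunt after a random wait.
; Once it settles frozen, a retriggerable delay arms DIE, which turns the player's view, disables movement and lunges at the camera.
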(event Custom|FLEE
  (bind _returnvalue (Math|Random|RandomFloatinRange 0.25 0.5))
  (bind _returnvalue_2 (Math|Random|RandomFloatinRange 0.25 0.75))
  (bind _skeletalmesh (Variables|Default|GetSkeletalMesh))
  (bind _skeletalmesh_2 (Variables|Default|GetSkeletalMesh))
  (bind _defaultsceneroot (Variables|Default|GetDefaultSceneRoot))
  (bind _defaultsceneroot_2 (Variables|Default|GetDefaultSceneRoot))
  (bind _skeletalmesh_3 (Variables|Default|GetSkeletalMesh))
  (bind _skeletalmesh_4 (Variables|Default|GetSkeletalMesh))
  (bind _defaultsceneroot_3 (Variables|Default|GetDefaultSceneRoot))
  (bind _returnvalue_3 (Transformation|GetWorldLocation _defaultsceneroot))
  (bind _returnvalue_4 (Transformation|GetWorldLocation _defaultsceneroot_3))
  ;[0 0.2291 1] FLEE
  (if (Variables|Default|GetRBBegin)
    _
    (else
      ;[1 0 0 0.5] GAME BEGIN
      (Variables|Default|SetRBBegin true)
      (bind _returnvalue_5 (Actor|GetActorOfClass "/Game/FirstPerson/Blueprints/BP_FirstPersonCharacter.BP_FirstPersonCharacter_C"))
      (Default|GAMEBEGIN _returnvalue_5)))
  (Utilities|FlowControl|Sequence
    (:then_0
      (goto _label Stop))
    (:then_1
      (if (not (Variables|Default|GetRBINVIN))
        (Variables|Default|SetRBINVIN true)
        (Variables|Default|SetRBKILL false)
        ;;[0 0 0 0.5] Sound
        (Audio|PlaySoundatLocation (.OutItem (Utilities|Array|Random (Utilities|Array|MakeArray "/Game/NotewatchContent/Audio/Sounds/Roboach1.Roboach1" "/Game/NotewatchContent/Audio/Sounds/Roboach2.Roboach2" "/Game/NotewatchContent/Audio/Sounds/Roboach3.Roboach3"))) _returnvalue_3 "0, 0, 0" (Math|Random|RandomFloatinRange 0.5 0.75) (Math|Random|RandomFloatinRange 1.0 2.0) 0.0 0 0 0 0)
        ;;[0 0 0 0.5] Sound
        (Audio|PlaySoundatLocation "/Game/NotewatchContent/Audio/Sounds/Brush.Brush" _returnvalue_3 "0, 0, 0" (Math|Random|RandomFloatinRange 0.5 0.75) (Math|Random|RandomFloatinRange 0.75 1.25) 0.0 0 0 0 0)
        (Components|Activation|Activate (Variables|Default|GetNiagara) true)
        (Components|Animation|PlayAnimation _skeletalmesh "/Game/NotewatchContent/Monsters/Roboach/Other/Idle.Idle" true)
        (Components|Timeline|SetPlayRate _skeletalmesh 5.0)
        (Components|MoveComponentTo _defaultsceneroot (+ (Variables|Default|GetStartLOC) "0.000000,0.000000,500.000000") (Math|Random|RandomRotator false) true false 0.5 true)
        (Utilities|FlowControl|Delay 1.0)
        (Variables|Default|SetStartLOC "0.000000,0.000000,-50000.000000")
        (Transformation|SetWorldLocation _defaultsceneroot (Variables|Default|GetStartLOC) false true)
        (Transformation|SetActorLocation (Variables|Default|GetStartLOC) false true)
        (Utilities|FlowControl|Delay (Math|Random|RandomFloatinRange 1e+01 2e+01))
        (Variables|Default|SetRBINVIN false)
        (Variables|Default|SetRBKILL false)
        (Components|Activation|Deactivate (Variables|Default|GetNiagara))
        ;[1 0.2527 0.8639] HUNT
        (Components|Animation|PlayAnimation _skeletalmesh_2 "/Game/NotewatchContent/Monsters/Roboach/Other/Idle.Idle" true)
        (Components|Timeline|SetPlayRate _skeletalmesh_2 1.0)
        (if (Variables|Default|GetRBBegin)
          (switch int (Math|Random|RandomIntegerinRange 0 2)
            (:0
              (Variables|Default|SetStartLOC (Variables|Default|GetLOC1))
              (Variables|Default|SetStartROT (Variables|Default|GetROT1)))
            (:1
              (Variables|Default|SetStartLOC (Variables|Default|GetLOC2))
              (Variables|Default|SetStartROT (Variables|Default|GetROT2)))
            (:2
              (Variables|Default|SetStartLOC (Variables|Default|GetLOC3))
              (Variables|Default|SetStartROT (Variables|Default|GetROT3))))
          (Transformation|SetActorLocationAndRotation (+ (Variables|Default|GetStartLOC) "0.000000,0.000000,500.000000") (Math|Random|RandomRotator false) false true)
          (Transformation|SetWorldLocation _defaultsceneroot_2 (+ (Variables|Default|GetStartLOC) "0.000000,0.000000,500.000000") false true)
          (Audio|PlaySoundatLocation "/Game/NotewatchContent/Audio/Sounds/Brush.Brush" _returnvalue_3 "0, 0, 0" (Math|Random|RandomFloatinRange 0.5 1.0) (Math|Random|RandomFloatinRange 1.5 2.0) 0.0 0 0 0 0)
          ;;[0 0 0 0.5] Sound
          (Audio|PlaySoundatLocation (.OutItem (Utilities|Array|Random (Utilities|Array|MakeArray "/Game/NotewatchContent/Audio/Sounds/Roboach1.Roboach1" "/Game/NotewatchContent/Audio/Sounds/Roboach2.Roboach2" "/Game/NotewatchContent/Audio/Sounds/Roboach3.Roboach3"))) _returnvalue_3 "0, 0, 0" _returnvalue_2 _returnvalue_2 0.0 0 0 0 0)
          (Components|MoveComponentTo _defaultsceneroot_2 (Variables|Default|GetStartLOC) (Variables|Default|GetStartROT) true true 2.0 true :!label _label)
          (Components|Animation|PlayAnimation _skeletalmesh_3 "/Game/NotewatchContent/Monsters/Roboach/Other/Freeze.Freeze" true)
          (Components|Timeline|SetPlayRate _skeletalmesh_3 0.25)
          (Variables|Default|SetRBKILL true)
          (Utilities|FlowControl|RetriggerableDelay (Math|Random|RandomFloatinRange 4e+01 4e+01))
          (if (Variables|Default|GetRBKILL)
            (CallFunction|DIE))
          (else
            ;[0.1138 0 1 0.5] HUNTFIRST
            (Variables|Default|SetStartLOC (Variables|Default|GetLOC3))
            (Variables|Default|SetStartROT (Variables|Default|GetROT3))
            (Transformation|SetActorLocationAndRotation (+ (Variables|Default|GetStartLOC) "0.000000,0.000000,500.000000") (Math|Random|RandomRotator false) false true)
            (Transformation|SetWorldLocation _defaultsceneroot_3 (+ (Variables|Default|GetStartLOC) "0.000000,0.000000,500.000000") false true)
            (Audio|PlaySoundatLocation "/Game/NotewatchContent/Audio/Sounds/Brush.Brush" _returnvalue_4 "0, 0, 0" (Math|Random|RandomFloatinRange 0.5 0.75) (Math|Random|RandomFloatinRange 1.5 2.0) 0.0 "/Game/NotewatchContent/Audio/Sounds/RinglingerAmbientAtten.RinglingerAmbientAtten" 0 0 0)
            (Audio|PlaySoundatLocation (.OutItem (Utilities|Array|Random (Utilities|Array|MakeArray "/Game/NotewatchContent/Audio/Sounds/Roboach1.Roboach1" "/Game/NotewatchContent/Audio/Sounds/Roboach2.Roboach2" "/Game/NotewatchContent/Audio/Sounds/Roboach3.Roboach3"))) _returnvalue_4 "0, 0, 0" _returnvalue _returnvalue 0.0 "/Game/NotewatchContent/Audio/Sounds/RinglingerAmbientAtten.RinglingerAmbientAtten" 0 0 0)
            (Components|MoveComponentTo _defaultsceneroot_3 (Variables|Default|GetStartLOC) (Variables|Default|GetStartROT) true true 2.0 true)
            (Components|Animation|PlayAnimation _skeletalmesh_4 "/Game/NotewatchContent/Monsters/Roboach/Other/Freeze.Freeze" true)
            (Components|Timeline|SetPlayRate _skeletalmesh_4 0.25)))))))

(event Custom|HUNT
  (bind _returnvalue (Math|Random|RandomFloatinRange 0.25 0.5))
  (bind _returnvalue_2 (Math|Random|RandomFloatinRange 0.25 0.75))
  (bind _skeletalmesh (Variables|Default|GetSkeletalMesh))
  (bind _defaultsceneroot (Variables|Default|GetDefaultSceneRoot))
  (bind _defaultsceneroot_2 (Variables|Default|GetDefaultSceneRoot))
  (bind _skeletalmesh_2 (Variables|Default|GetSkeletalMesh))
  (bind _skeletalmesh_3 (Variables|Default|GetSkeletalMesh))
  (bind _defaultsceneroot_3 (Variables|Default|GetDefaultSceneRoot))
  (bind _returnvalue_3 (Transformation|GetWorldLocation _defaultsceneroot))
  (bind _returnvalue_4 (Transformation|GetWorldLocation _defaultsceneroot_3))
  ;[1 0.2527 0.8639] HUNT
  (if (not (Variables|Default|GetRBINVIN))
    (Utilities|FlowControl|Delay (Math|Random|RandomFloatinRange 1.0 2.0))
    (Components|Animation|PlayAnimation _skeletalmesh "/Game/NotewatchContent/Monsters/Roboach/Other/Idle.Idle" true)
    (Components|Timeline|SetPlayRate _skeletalmesh 1.0)
    (if (Variables|Default|GetRBBegin)
      (switch int (Math|Random|RandomIntegerinRange 0 2)
        (:0
          (Variables|Default|SetStartLOC (Variables|Default|GetLOC1))
          (Variables|Default|SetStartROT (Variables|Default|GetROT1)))
        (:1
          (Variables|Default|SetStartLOC (Variables|Default|GetLOC2))
          (Variables|Default|SetStartROT (Variables|Default|GetROT2)))
        (:2
          (Variables|Default|SetStartLOC (Variables|Default|GetLOC3))
          (Variables|Default|SetStartROT (Variables|Default|GetROT3))))
      (Transformation|SetActorLocationAndRotation (+ (Variables|Default|GetStartLOC) "0.000000,0.000000,500.000000") (Math|Random|RandomRotator false) false true)
      (Transformation|SetWorldLocation _defaultsceneroot_2 (+ (Variables|Default|GetStartLOC) "0.000000,0.000000,500.000000") false true)
      (Audio|PlaySoundatLocation "/Game/NotewatchContent/Audio/Sounds/Brush.Brush" _returnvalue_3 "0, 0, 0" (Math|Random|RandomFloatinRange 0.5 1.0) (Math|Random|RandomFloatinRange 1.5 2.0) 0.0 0 0 0 0)
      ;[0 0.2291 1] FLEE
      ;;[0 0 0 0.5] Sound
      (Audio|PlaySoundatLocation (.OutItem (Utilities|Array|Random (Utilities|Array|MakeArray "/Game/NotewatchContent/Audio/Sounds/Roboach1.Roboach1" "/Game/NotewatchContent/Audio/Sounds/Roboach2.Roboach2" "/Game/NotewatchContent/Audio/Sounds/Roboach3.Roboach3"))) _returnvalue_3 "0, 0, 0" _returnvalue_2 _returnvalue_2 0.0 0 0 0 0)
      (Components|MoveComponentTo _defaultsceneroot_2 (Variables|Default|GetStartLOC) (Variables|Default|GetStartROT) true true 2.0 true)
      (Components|Animation|PlayAnimation _skeletalmesh_2 "/Game/NotewatchContent/Monsters/Roboach/Other/Freeze.Freeze" true)
      (Components|Timeline|SetPlayRate _skeletalmesh_2 0.25)
      (Variables|Default|SetRBKILL true)
      (Utilities|FlowControl|RetriggerableDelay (Math|Random|RandomFloatinRange 4e+01 4e+01))
      (if (Variables|Default|GetRBKILL)
        (CallFunction|DIE))
      (else
        ;[0.1138 0 1 0.5] HUNTFIRST
        (Variables|Default|SetStartLOC (Variables|Default|GetLOC3))
        (Variables|Default|SetStartROT (Variables|Default|GetROT3))
        (Transformation|SetActorLocationAndRotation (+ (Variables|Default|GetStartLOC) "0.000000,0.000000,500.000000") (Math|Random|RandomRotator false) false true)
        (Transformation|SetWorldLocation _defaultsceneroot_3 (+ (Variables|Default|GetStartLOC) "0.000000,0.000000,500.000000") false true)
        (Audio|PlaySoundatLocation "/Game/NotewatchContent/Audio/Sounds/Brush.Brush" _returnvalue_4 "0, 0, 0" (Math|Random|RandomFloatinRange 0.5 0.75) (Math|Random|RandomFloatinRange 1.5 2.0) 0.0 "/Game/NotewatchContent/Audio/Sounds/RinglingerAmbientAtten.RinglingerAmbientAtten" 0 0 0)
        (Audio|PlaySoundatLocation (.OutItem (Utilities|Array|Random (Utilities|Array|MakeArray "/Game/NotewatchContent/Audio/Sounds/Roboach1.Roboach1" "/Game/NotewatchContent/Audio/Sounds/Roboach2.Roboach2" "/Game/NotewatchContent/Audio/Sounds/Roboach3.Roboach3"))) _returnvalue_4 "0, 0, 0" _returnvalue _returnvalue 0.0 "/Game/NotewatchContent/Audio/Sounds/RinglingerAmbientAtten.RinglingerAmbientAtten" 0 0 0)
        (Components|MoveComponentTo _defaultsceneroot_3 (Variables|Default|GetStartLOC) (Variables|Default|GetStartROT) true true 2.0 true)
        (Components|Animation|PlayAnimation _skeletalmesh_3 "/Game/NotewatchContent/Monsters/Roboach/Other/Freeze.Freeze" true)
        (Components|Timeline|SetPlayRate _skeletalmesh_3 0.25)))))

(event Custom|DIE
  (bind _returnvalue (Math|Random|RandomFloatinRange 1.5 1.5))
  (bind _returnvalue_2 (Math|Random|RandomFloatinRange 0.75 1.25))
  (bind _defaultsceneroot (Variables|Default|GetDefaultSceneRoot))
  (bind _returnvalue_3 (Transformation|GetWorldLocation _defaultsceneroot))
  ;[1 0 0.005053] Kill
  (Variables|Default|SetRBINVIN true)
  (bind _returnvalue_4 (Actor|GetActorOfClass "/Game/FirstPerson/Blueprints/BP_FirstPersonCharacter.BP_FirstPersonCharacter_C"))
  (Pawn|SetControlRotation (Game|GetPlayerController (Variables|/Script/Engine.Pawn|GetPlayerState _returnvalue_4)) (Math|Rotator|FindLookatRotation (Transformation|GetWorldLocation (Variables|/Game/FirstPerson/Blueprints/BP_FirstPersonCharacter.BP_FirstPersonCharacter_C|GetFirstPersonCamera _returnvalue_4)) _returnvalue_3))
  (Pawn|Components|CharacterMovement|DisableMovement (Variables|/Script/Engine.Character|GetCharacterMovement _returnvalue_4))
  ;;[0 0 0 0.5] Sound
  (Audio|PlaySoundatLocation (.OutItem (Utilities|Array|Random (Utilities|Array|MakeArray "/Game/NotewatchContent/Audio/Sounds/Roboach1.Roboach1" "/Game/NotewatchContent/Audio/Sounds/Roboach2.Roboach2" "/Game/NotewatchContent/Audio/Sounds/Roboach3.Roboach3"))) (Transformation|GetWorldLocation (Variables|/Game/FirstPerson/Blueprints/BP_FirstPersonCharacter.BP_FirstPersonCharacter_C|GetFirstPersonCamera _returnvalue_4)) "0, 0, 0" _returnvalue _returnvalue_2 0.0 0 0 0 0)
  (Audio|PlaySoundatLocation "/Game/NotewatchContent/Audio/Sounds/RoboachRoar.RoboachRoar" _returnvalue_3 "0, 0, 0" _returnvalue _returnvalue_2 0.0 0 0 0 0)
  (Components|MoveComponentTo (Variables|Default|GetDefaultSceneRoot) (Transformation|GetWorldLocation (Variables|/Game/FirstPerson/Blueprints/BP_FirstPersonCharacter.BP_FirstPersonCharacter_C|GetFirstPersonCamera _returnvalue_4)) (Math|Random|RandomRotator true) false false 0.5 false)
  (Default|DIE _returnvalue_4))

(fn ConstructionScript)