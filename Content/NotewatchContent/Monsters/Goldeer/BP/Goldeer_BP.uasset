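; Goldeer monster actor that runs in to one of three preset spots, idles, and retreats when told to flee or die.
; FLEE drops it far below the map, waits, then rejoins HUNT's approach, teleporting to an offset start and gliding in via MoveComponentTo.
; After arrival, and on DIE, which freezes its pose before fleeing, it hides FlashBeacon_BP and briefly switches it off with a flashlight sound.
; A GDFLEEING flag guards re-entry.
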(event Custom|FLEE
  (bind _returnvalue (Math|Random|RandomFloatinRange 0.0 0.0))
  (bind _skeletalmesh (Variables|Default|GetSkeletalMesh))
  (bind _defaultsceneroot (Variables|Default|GetDefaultSceneRoot))
  (bind _skeletalmesh_2 (Variables|Default|GetSkeletalMesh))
  ;[0 0.2291 1] FLEE
  (if (not (Variables|Default|GetGDFLEEING))
    (Variables|Default|SetGDFLEEING true)
    (Utilities|FlowControl|Sequence
      (:then_0
        (goto _label_2 Stop))
      (:then_1
        (Variables|Default|SetGDKILL false)
        ;;[0 0 0 0.5] Sound
        (Audio|PlaySoundatLocation (.OutItem (Utilities|Array|Random (Utilities|Array|MakeArray "/Game/NotewatchContent/Audio/Sounds/Goldeer1.Goldeer1" "/Game/NotewatchContent/Audio/Sounds/Goldeer2.Goldeer2" "/Game/NotewatchContent/Audio/Sounds/Goldeer3.Goldeer3"))) "0, 0, 0" "0, 0, 0" (Math|Random|RandomFloatinRange 0.0 0.0) (Math|Random|RandomFloatinRange 0.75 1.25) 0.0 "/Game/NotewatchContent/Audio/Sounds/RinglingerAmbientAtten.RinglingerAmbientAtten" 0 0 0)
        (Variables|Default|SetStartLOC "0.000000,0.000000,-50000.000000")
        (Transformation|SetWorldLocation _defaultsceneroot (Variables|Default|GetStartLOC) false true)
        (Transformation|SetActorLocation (Variables|Default|GetStartLOC) false true)
        (Utilities|FlowControl|Delay (Math|Random|RandomFloatinRange 1e+01 2e+01))
        (Variables|Default|SetGDFLEEING false)
        (Variables|Default|SetGDKILL false)
        ;[1 0.2527 0.8639] HUNT
        (Components|Animation|PlayAnimation _skeletalmesh "/Game/NotewatchContent/Monsters/Goldeer/Other/Run.Run" true)
        (Components|Timeline|SetPlayRate _skeletalmesh 0.5)
        (switch int (Math|Random|RandomIntegerinRange 0 2)
          (:0
            (Variables|Default|SetStartLOC (Variables|Default|GetLOC1))
            (Variables|Default|SetStartROT (Variables|Default|GetROT1))
            (Transformation|SetActorLocationAndRotation (+ (Variables|Default|GetStartLOC) "-750.000000,10000.000000,1000.000000") "0.000000,90.000000,0.000000" false true :!label _label)
            (Transformation|SetWorldLocation _defaultsceneroot (+ (Variables|Default|GetStartLOC) "-750.000000,10000.000000,1000.000000") false true))
          (:1
            (Variables|Default|SetStartLOC (Variables|Default|GetLOC2))
            (Variables|Default|SetStartROT (Variables|Default|GetROT2))
            (Transformation|SetActorLocationAndRotation (+ (Variables|Default|GetStartLOC) "-750.000000,10000.000000,500.000000") "0.000000,-50.000000,0.000000" false true)
            (Transformation|SetWorldLocation (Variables|Default|GetDefaultSceneRoot) (+ (Variables|Default|GetStartLOC) "-750.000000,10000.000000,500.000000") false true))
          (:2
            (Variables|Default|SetStartLOC (Variables|Default|GetLOC3))
            (Variables|Default|SetStartROT (Variables|Default|GetROT3))
            (goto _label)))
        ;;[0 0 0 0.5] Sound
        (Audio|PlaySoundatLocation (.OutItem (Utilities|Array|Random (Utilities|Array|MakeArray "/Game/NotewatchContent/Audio/Sounds/Goldeer1.Goldeer1" "/Game/NotewatchContent/Audio/Sounds/Goldeer2.Goldeer2" "/Game/NotewatchContent/Audio/Sounds/Goldeer3.Goldeer3"))) (Transformation|GetWorldLocation (Variables|Default|GetDefaultSceneRoot)) "0, 0, 0" _returnvalue _returnvalue 0.0 "/Game/NotewatchContent/Audio/Sounds/RinglingerAmbientAtten.RinglingerAmbientAtten" 0 0 0)
        (Components|MoveComponentTo _defaultsceneroot (Variables|Default|GetStartLOC) "0.000000,5.000000,0.000000" true false 5.0 true :!label _label_2)
        (Components|Timeline|SetPlayRate _skeletalmesh_2 0.5)
        (Components|MoveComponentTo _defaultsceneroot (Variables|Default|GetStartLOC) (Variables|Default|GetStartROT) false false 1.0 true)
        (Components|Animation|PlayAnimation _skeletalmesh_2 "/Game/NotewatchContent/Monsters/Goldeer/Other/Idle.Idle" true)
        (Components|Timeline|SetPlayRate _skeletalmesh_2 0.25)
        (Variables|Default|SetGDFLEEING false)
        ;[1 0.9227 0 0.5] Vanish
        (Utilities|FlowControl|Delay (Math|Random|RandomFloatinRange 1e+01 2e+01))
        (bind _returnvalue_2 (Actor|GetActorOfClass "/Game/NotewatchContent/Lights/FlashBeacon_BP.FlashBeacon_BP_C"))
        (Utilities|FlowControl|Delay (Math|Random|RandomFloatinRange 1.0 1e+01))
        (Audio|PlaySound2D "/Game/NotewatchContent/Audio/Sounds/Flashlight.Flashlight" 3.0 2.0 0.0 0 0)
        (Variables|/Game/NotewatchContent/Lights/FlashBeacon_BP.FlashBeacon_BP_C|SetON _returnvalue_2 false)
        (Rendering|SetActorHiddenInGame _returnvalue_2 true)
        (Utilities|FlowControl|Sequence
          (:then_1
            (Utilities|FlowControl|RetriggerableDelay (Math|Random|RandomFloatinRange 0.5 0.5))
            (Variables|/Game/NotewatchContent/Lights/FlashBeacon_BP.FlashBeacon_BP_C|SetON _returnvalue_2 true)))))))

(event Custom|HUNT
  (bind _returnvalue (Math|Random|RandomFloatinRange 0.0 0.0))
  (bind _skeletalmesh (Variables|Default|GetSkeletalMesh))
  (bind _defaultsceneroot (Variables|Default|GetDefaultSceneRoot))
  (bind _skeletalmesh_2 (Variables|Default|GetSkeletalMesh))
  ;[1 0.2527 0.8639] HUNT
  (if (not (Variables|Default|GetGDFLEEING))
    (Variables|Default|SetGDFLEEING true)
    (Utilities|FlowControl|Delay (Math|Random|RandomFloatinRange 2e+02 4e+02))
    (Components|Animation|PlayAnimation _skeletalmesh "/Game/NotewatchContent/Monsters/Goldeer/Other/Run.Run" true)
    (Components|Timeline|SetPlayRate _skeletalmesh 0.5)
    (switch int (Math|Random|RandomIntegerinRange 0 2)
      (:0
        (Variables|Default|SetStartLOC (Variables|Default|GetLOC1))
        (Variables|Default|SetStartROT (Variables|Default|GetROT1))
        (Transformation|SetActorLocationAndRotation (+ (Variables|Default|GetStartLOC) "-750.000000,10000.000000,1000.000000") "0.000000,90.000000,0.000000" false true :!label _label)
        (Transformation|SetWorldLocation _defaultsceneroot (+ (Variables|Default|GetStartLOC) "-750.000000,10000.000000,1000.000000") false true))
      (:1
        (Variables|Default|SetStartLOC (Variables|Default|GetLOC2))
        (Variables|Default|SetStartROT (Variables|Default|GetROT2))
        (Transformation|SetActorLocationAndRotation (+ (Variables|Default|GetStartLOC) "-750.000000,10000.000000,500.000000") "0.000000,-50.000000,0.000000" false true)
        (Transformation|SetWorldLocation (Variables|Default|GetDefaultSceneRoot) (+ (Variables|Default|GetStartLOC) "-750.000000,10000.000000,500.000000") false true))
      (:2
        (Variables|Default|SetStartLOC (Variables|Default|GetLOC3))
        (Variables|Default|SetStartROT (Variables|Default|GetROT3))
        (goto _label)))
    ;[0 0.2291 1] FLEE
    ;;[0 0 0 0.5] Sound
    (Audio|PlaySoundatLocation (.OutItem (Utilities|Array|Random (Utilities|Array|MakeArray "/Game/NotewatchContent/Audio/Sounds/Goldeer1.Goldeer1" "/Game/NotewatchContent/Audio/Sounds/Goldeer2.Goldeer2" "/Game/NotewatchContent/Audio/Sounds/Goldeer3.Goldeer3"))) (Transformation|GetWorldLocation (Variables|Default|GetDefaultSceneRoot)) "0, 0, 0" _returnvalue _returnvalue 0.0 "/Game/NotewatchContent/Audio/Sounds/RinglingerAmbientAtten.RinglingerAmbientAtten" 0 0 0)
    (Components|MoveComponentTo _defaultsceneroot (Variables|Default|GetStartLOC) "0.000000,5.000000,0.000000" true false 5.0 true)
    (Components|Timeline|SetPlayRate _skeletalmesh_2 0.5)
    (Components|MoveComponentTo _defaultsceneroot (Variables|Default|GetStartLOC) (Variables|Default|GetStartROT) false false 1.0 true)
    (Components|Animation|PlayAnimation _skeletalmesh_2 "/Game/NotewatchContent/Monsters/Goldeer/Other/Idle.Idle" true)
    (Components|Timeline|SetPlayRate _skeletalmesh_2 0.25)
    (Variables|Default|SetGDFLEEING false)
    ;[1 0.9227 0 0.5] Vanish
    (Utilities|FlowControl|Delay (Math|Random|RandomFloatinRange 1e+01 2e+01))
    (bind _returnvalue_2 (Actor|GetActorOfClass "/Game/NotewatchContent/Lights/FlashBeacon_BP.FlashBeacon_BP_C"))
    (Utilities|FlowControl|Delay (Math|Random|RandomFloatinRange 1.0 1e+01))
    (Audio|PlaySound2D "/Game/NotewatchContent/Audio/Sounds/Flashlight.Flashlight" 3.0 2.0 0.0 0 0)
    (Variables|/Game/NotewatchContent/Lights/FlashBeacon_BP.FlashBeacon_BP_C|SetON _returnvalue_2 false)
    (Rendering|SetActorHiddenInGame _returnvalue_2 true)
    (Utilities|FlowControl|Sequence
      (:then_1
        (Utilities|FlowControl|RetriggerableDelay (Math|Random|RandomFloatinRange 0.5 0.5))
        (Variables|/Game/NotewatchContent/Lights/FlashBeacon_BP.FlashBeacon_BP_C|SetON _returnvalue_2 true)))))

(event Custom|DIE
  (bind _returnvalue (Math|Random|RandomFloatinRange 0.0 0.0))
  (bind _skeletalmesh (Variables|Default|GetSkeletalMesh))
  (bind _defaultsceneroot (Variables|Default|GetDefaultSceneRoot))
  (bind _defaultsceneroot_2 (Variables|Default|GetDefaultSceneRoot))
  (bind _skeletalmesh_2 (Variables|Default|GetSkeletalMesh))
  (bind _skeletalmesh_3 (Variables|Default|GetSkeletalMesh))
  (bind _returnvalue_2 (Transformation|GetWorldLocation _defaultsceneroot_2))
  ;[1 0 0.005053] DEATH
  ;;[0 0 0 0.5] Sound
  (Audio|PlaySoundatLocation (.OutItem (Utilities|Array|Random (Utilities|Array|MakeArray "/Game/NotewatchContent/Audio/Sounds/Goldeer1.Goldeer1" "/Game/NotewatchContent/Audio/Sounds/Goldeer2.Goldeer2" "/Game/NotewatchContent/Audio/Sounds/Goldeer3.Goldeer3"))) _returnvalue_2 "0, 0, 0" (Math|Random|RandomFloatinRange 0.0 0.025) (Math|Random|RandomFloatinRange 1.25 1.5) 0.0 "/Game/NotewatchContent/Audio/Sounds/RinglingerAmbientAtten.RinglingerAmbientAtten" 0 0 0)
  (Components|Timeline|SetPlayRate _skeletalmesh_2 0.0)
  (Components|Animation|SetPosition _skeletalmesh_2 2.5 true)
  (bind _returnvalue_3 (Actor|GetActorOfClass "/Game/NotewatchContent/Lights/FlashBeacon_BP.FlashBeacon_BP_C"))
  (Utilities|FlowControl|Delay (Math|Random|RandomFloatinRange 1.0 1e+01))
  (Audio|PlaySound2D "/Game/NotewatchContent/Audio/Sounds/Flashlight.Flashlight" 3.0 0.25 0.4 0 0)
  (Variables|/Game/NotewatchContent/Lights/FlashBeacon_BP.FlashBeacon_BP_C|SetON _returnvalue_3 false)
  (Rendering|SetActorHiddenInGame _returnvalue_3 true)
  (Utilities|FlowControl|Sequence
    (:then_0
      ;[0 0.2291 1] FLEE
      (Variables|Default|SetGDFLEEING true)
      (Utilities|FlowControl|Sequence
        (:then_0
          (goto _label_2 Stop))
        (:then_1
          (Variables|Default|SetGDKILL false)
          ;;[0 0 0 0.5] Sound
          (Audio|PlaySoundatLocation (.OutItem (Utilities|Array|Random (Utilities|Array|MakeArray "/Game/NotewatchContent/Audio/Sounds/Goldeer1.Goldeer1" "/Game/NotewatchContent/Audio/Sounds/Goldeer2.Goldeer2" "/Game/NotewatchContent/Audio/Sounds/Goldeer3.Goldeer3"))) "0, 0, 0" "0, 0, 0" (Math|Random|RandomFloatinRange 0.0 0.0) (Math|Random|RandomFloatinRange 0.75 1.25) 0.0 "/Game/NotewatchContent/Audio/Sounds/RinglingerAmbientAtten.RinglingerAmbientAtten" 0 0 0)
          (Variables|Default|SetStartLOC "0.000000,0.000000,-50000.000000")
          (Transformation|SetWorldLocation _defaultsceneroot (Variables|Default|GetStartLOC) false true)
          (Transformation|SetActorLocation (Variables|Default|GetStartLOC) false true)
          (Utilities|FlowControl|Delay (Math|Random|RandomFloatinRange 1e+01 2e+01))
          (Variables|Default|SetGDFLEEING false)
          (Variables|Default|SetGDKILL false)
          ;[1 0.2527 0.8639] HUNT
          (Components|Animation|PlayAnimation _skeletalmesh "/Game/NotewatchContent/Monsters/Goldeer/Other/Run.Run" true)
          (Components|Timeline|SetPlayRate _skeletalmesh 0.5)
          (switch int (Math|Random|RandomIntegerinRange 0 2)
            (:0
              (Variables|Default|SetStartLOC (Variables|Default|GetLOC1))
              (Variables|Default|SetStartROT (Variables|Default|GetROT1))
              (Transformation|SetActorLocationAndRotation (+ (Variables|Default|GetStartLOC) "-750.000000,10000.000000,1000.000000") "0.000000,90.000000,0.000000" false true :!label _label)
              (Transformation|SetWorldLocation _defaultsceneroot (+ (Variables|Default|GetStartLOC) "-750.000000,10000.000000,1000.000000") false true))
            (:1
              (Variables|Default|SetStartLOC (Variables|Default|GetLOC2))
              (Variables|Default|SetStartROT (Variables|Default|GetROT2))
              (Transformation|SetActorLocationAndRotation (+ (Variables|Default|GetStartLOC) "-750.000000,10000.000000,500.000000") "0.000000,-50.000000,0.000000" false true)
              (Transformation|SetWorldLocation (Variables|Default|GetDefaultSceneRoot) (+ (Variables|Default|GetStartLOC) "-750.000000,10000.000000,500.000000") false true))
            (:2
              (Variables|Default|SetStartLOC (Variables|Default|GetLOC3))
              (Variables|Default|SetStartROT (Variables|Default|GetROT3))
              (goto _label)))
          ;;[0 0 0 0.5] Sound
          (Audio|PlaySoundatLocation (.OutItem (Utilities|Array|Random (Utilities|Array|MakeArray "/Game/NotewatchContent/Audio/Sounds/Goldeer1.Goldeer1" "/Game/NotewatchContent/Audio/Sounds/Goldeer2.Goldeer2" "/Game/NotewatchContent/Audio/Sounds/Goldeer3.Goldeer3"))) _returnvalue_2 "0, 0, 0" _returnvalue _returnvalue 0.0 "/Game/NotewatchContent/Audio/Sounds/RinglingerAmbientAtten.RinglingerAmbientAtten" 0 0 0)
          (Components|MoveComponentTo _defaultsceneroot (Variables|Default|GetStartLOC) "0.000000,5.000000,0.000000" true false 5.0 true :!label _label_2)
          (Components|Timeline|SetPlayRate _skeletalmesh_3 0.5)
          (Components|MoveComponentTo _defaultsceneroot (Variables|Default|GetStartLOC) (Variables|Default|GetStartROT) false false 1.0 true)
          (Components|Animation|PlayAnimation _skeletalmesh_3 "/Game/NotewatchContent/Monsters/Goldeer/Other/Idle.Idle" true)
          (Components|Timeline|SetPlayRate _skeletalmesh_3 0.25)
          (Variables|Default|SetGDFLEEING false)
          ;[1 0.9227 0 0.5] Vanish
          (Utilities|FlowControl|Delay (Math|Random|RandomFloatinRange 1e+01 2e+01))
          (bind _returnvalue_4 (Actor|GetActorOfClass "/Game/NotewatchContent/Lights/FlashBeacon_BP.FlashBeacon_BP_C"))
          (Utilities|FlowControl|Delay (Math|Random|RandomFloatinRange 1.0 1e+01))
          (Audio|PlaySound2D "/Game/NotewatchContent/Audio/Sounds/Flashlight.Flashlight" 3.0 2.0 0.0 0 0)
          (Variables|/Game/NotewatchContent/Lights/FlashBeacon_BP.FlashBeacon_BP_C|SetON _returnvalue_4 false)
          (Rendering|SetActorHiddenInGame _returnvalue_4 true)
          (Utilities|FlowControl|Sequence
            (:then_1
              (Utilities|FlowControl|RetriggerableDelay (Math|Random|RandomFloatinRange 0.5 0.5))
              (Variables|/Game/NotewatchContent/Lights/FlashBeacon_BP.FlashBeacon_BP_C|SetON _returnvalue_4 true))))))
    (:then_1
      (Utilities|FlowControl|RetriggerableDelay (Math|Random|RandomFloatinRange 1e+01 1e+01))
      (Variables|/Game/NotewatchContent/Lights/FlashBeacon_BP.FlashBeacon_BP_C|SetON _returnvalue_3 true))))

(fn ConstructionScript)